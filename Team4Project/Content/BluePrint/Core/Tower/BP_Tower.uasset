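; Defense tower actor for all tower types, configured from TowerType data at construction: level, stats, grid-scaled range and preview or placed materials.
; Its range box tracks enemies or towers according to targetable types.
; Towers with an attack rate loop bullet shots using a polling timer and delay.
; Zero-rate towers apply effects: NK Spreader modifies enemy speed and requests removal after enough entries, while Epinephrine Ejector boosts nearby towers' attack rate.
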(event `AnimTest`
  (bind _geometrycache (`self.GeometryCache`))
  (`SceneComponent.SetVisibility` _geometrycache true false)
  (`GeometryCacheComponent.Play` _geometrycache))

(event `self.ReceiveBeginPlay`
  (set `self.TotalNumOfEnemyEnterTheAttackRange` 0)
  (if (!= (`self.CurrentAttackRate`) 0.0)
    (`self.StartToCheckEnemyAndShoot`)
    (else
      (switch `/Game/BluePrint/Core/Tower/Utilities/Enum_TowerType` (`self.TowerType`)
        (:`NewEnumerator1`
          (`self.RefreshEffectRangeOverlappedTowers`))))))

(event `self.AttackRangeCollisionBox.OnComponentBeginOverlap`
  (params (OverlappedComponent :type "PrimitiveComponent Object Reference") (OtherActor :type "Actor Object Reference") (OtherComp :type "PrimitiveComponent Object Reference") (OtherBodyIndex :type Integer) (bFromSweep :type Boolean) (SweepResult :type "HitResult Structure (by ref)"))
  (bind ((`AttackableTargetType_42_07615D6F474C4A43AE8D2ABA95AEE68A` _attackabletargettype)) (break `/Game/BluePrint/Core/Tower/Utilities/S_DefenseTowerData` (`self.TowerData`)))
  (if (`KismetArrayLibrary.Array_Contains` _attackabletargettype "NewEnumerator0")
    (bind _asbp_unit_master_enemy (cast `/Game/BluePrint/Core/Character/BP_UnitMaster_Enemy` OtherActor)
      (:`then`
        (add `/Game/BluePrint/Core/Character/BP_UnitMaster_Enemy.OnEnemyNeedToRemoveFromCombat` _asbp_unit_master_enemy (`|CreateDelegate` :!event `OnEnemyNeedToRemoveFromCombat`))
        (`KismetArrayLibrary.Array_Add` (`self.UnitEnemyInAttackRange`) _asbp_unit_master_enemy)
        (`/Engine/EditorBlueprintResources/StandardMacros.IncrementInt` (`self.TotalNumOfEnemyEnterTheAttackRange`)
          (:`  `
            (if (!= (`self.CurrentAttackRate`) 0.0)
              (if (not (`self.IsInAttackingLoop`))
                (set `self.IsInAttackingLoop` true)
                (`self.AttackEnemyBaseOnTowerType`))
              (else
                (`self.AttackEnemyBaseOnTowerType`))))))
      (:`CastFailed`
        (bind _asbp_tower (cast `/Game/BluePrint/Core/Tower/BP_Tower` OtherActor :!label _label))
        (if (!= _asbp_tower self)
          (if (== (`self.CurrentAttackRate`) 0.0)
            (`KismetSystemLibrary.PrintString` "AddTowerInMyEffectRange" true true (struct :`R` 0.018419 :`B` 1.0 :`A` 1.0) 5.0)
            (`self.AddTowerInEffectRange` _asbp_tower)
            (elif (== (`/Game/BluePrint/Core/Tower/BP_Tower.CurrentAttackRate` _asbp_tower) 0.0)
              (`KismetSystemLibrary.PrintString` "AddTowerInOtherEffectRange" true true (struct :`R` 0.018419 :`B` 1.0 :`A` 1.0) 5.0)
              (`self.AddTowerInEffectRange` _asbp_tower self))))))
    (elif (`KismetArrayLibrary.Array_Contains` _attackabletargettype "NewEnumerator1")
      (goto _label))))

(event `self.AttackRangeCollisionBox.OnComponentEndOverlap`
  (params (OverlappedComponent :type "PrimitiveComponent Object Reference") (OtherActor :type "Actor Object Reference") (OtherComp :type "PrimitiveComponent Object Reference") (OtherBodyIndex :type Integer))
  (bind ((`AttackableTargetType_42_07615D6F474C4A43AE8D2ABA95AEE68A` _attackabletargettype)) (break `/Game/BluePrint/Core/Tower/Utilities/S_DefenseTowerData` (`self.TowerData`)))
  (if (`KismetArrayLibrary.Array_Contains` _attackabletargettype "NewEnumerator0")
    (bind _asbp_unit_master_enemy (cast `/Game/BluePrint/Core/Character/BP_UnitMaster_Enemy` OtherActor))
    (if (`KismetArrayLibrary.Array_Contains` (`self.UnitEnemyInAttackRange`) _asbp_unit_master_enemy)
      (`KismetArrayLibrary.Array_RemoveItem` (`self.UnitEnemyInAttackRange`) _asbp_unit_master_enemy)
      (`KismetArrayLibrary.Array_RemoveItem` (`self.EffectedEnemyRecord`) _asbp_unit_master_enemy))
    (elif (`KismetArrayLibrary.Array_Contains` _attackabletargettype "NewEnumerator1")
      (bind _asbp_tower (cast `/Game/BluePrint/Core/Tower/BP_Tower` OtherActor))
      (`self.RemoveTowerFromEffectRange` _asbp_tower))))

(event `StartToCheckEnemyAndShoot`
  (bind _returnvalue (`KismetSystemLibrary.K2_SetTimerDelegate` (delegate `IsTowerInAttackingLoop`) 0.2 true))
  (set `self.AttackTimer` _returnvalue))

(event `IsTowerInAttackingLoop`
  (if (`self.IsInAttackingLoop`)
    _
    (elif (and (!= (`self.CurrentAttackRate`) 0.0) (> (`KismetArrayLibrary.Array_Length` (`self.UnitEnemyInAttackRange`)) 0))
      (set `self.IsInAttackingLoop` true)
      (`self.AttackEnemyBaseOnTowerType`)
      (else
        (set `self.IsInAttackingLoop` false)))))

(event `FinishedOnceAttack`
  (`KismetSystemLibrary.Delay` (/ 1.0 (`self.CurrentAttackRate`)))
  (`self.AttackEnemyBaseOnTowerType`))

(event `AttackEnemyBaseOnTowerType`
  (if (> (`KismetArrayLibrary.Array_Length` (`self.UnitEnemyInAttackRange`)) 0)
    (if (!= (`self.CurrentAttackRate`) 0.0)
      (set `self.CurrentTargetEnemyIndex` 0)
      (bind _output_get (set `self.AimingEnemy` (`|GetArrayItem` (`self.UnitEnemyInAttackRange`) (`self.CurrentTargetEnemyIndex`)) :!label _label))
      (`/Engine/EditorBlueprintResources/StandardMacros.IsValid` _output_get
        (:`Is Valid`
          (set `self.IsInAttackingLoop` true)
          (switch `/Game/BluePrint/Core/Tower/Utilities/Enum_TowerType` (`self.TowerType`)
            (:`NewEnumerator0`
              (`|SpawnActorFromClass` "/Game/BluePrint/Core/Tower/BP_TowerBullet.BP_TowerBullet_C" (`KismetMathLibrary.MakeTransform` (`self.K2_GetActorLocation`)) "AlwaysSpawn" "MultiplyWithRoot" null (`self.AimingEnemy`) (`self.CurrentAttackDamageOrEffectPercent`) null)
              (`self.FinishedOnceAttack`))))
        (:`Is Not Valid`
          (`KismetSystemLibrary.PrintString` "NotValidEnemy")
          (bind _result (`/Engine/EditorBlueprintResources/StandardMacros.IncrementInt` (`self.CurrentTargetEnemyIndex`))
            (:`  `
              (if (< _result (`KismetArrayLibrary.Array_Length` (`self.UnitEnemyInAttackRange`)))
                (goto _label)
                (else
                  (set `self.IsInAttackingLoop` false)))))))
      (else
        (switch `/Game/BluePrint/Core/Tower/Utilities/Enum_TowerType` (`self.TowerType`)
          (:`NewEnumerator2`
            (set `self.AimingEnemy` (`self.GetAnEnemyNotEffected`))
            (`/Game/BluePrint/Core/Character/BP_UnitMaster_Enemy.ModifierCurrentMoveSpeed` (`self.AimingEnemy`) -999.0 (`self.CurrentAttackDamageOrEffectPercent`))
            (`KismetArrayLibrary.Array_Add` (`self.EffectedEnemyRecord`) (`self.AimingEnemy`))
            (if (> (`self.TotalNumOfEnemyEnterTheAttackRange`) 10)
              (`self.OnTowerNeedToBeAutoRemovedFromCombatAfterCompletedEffectNum` self))))))
    (else
      (set `self.IsInAttackingLoop` false))))

(fn `AddBuffOrDebuffFromEffectTower`
  (params (EffectTower :type "/Game/BluePrint/Core/Tower/BP_Tower Object Reference"))
  (switch `/Game/BluePrint/Core/Tower/Utilities/Enum_TowerType` (`/Game/BluePrint/Core/Tower/BP_Tower.TowerType` EffectTower)
    (:`NewEnumerator1`
      (`self.ModifierAttackRate` 1.5))))

(fn `AddTowerInEffectRange`
  (params (NewTower :type "/Game/BluePrint/Core/Tower/BP_Tower Object Reference"))
  (bind _newtower (`local.NewTower`))
  (if (not (`KismetArrayLibrary.Array_Contains` (`self.TowerInEffectRange`) (`local.NewTower`)))
    (`KismetArrayLibrary.Array_Add` (`self.TowerInEffectRange`) _newtower)
    (`KismetArrayLibrary.Array_Add` (`/Game/BluePrint/Core/Tower/BP_Tower.ParentTowerOfBuff` _newtower) self)
    (`self.AddBuffOrDebuffFromEffectTower` _newtower self)
    (else
      (`KismetSystemLibrary.PrintString` "AlreadyInEffectRange"))))

(fn `CheckIsTargetTowerInEffectRange`
  (params (TargetTower :type "/Game/BluePrint/Core/Tower/BP_Tower Object Reference"))
  (returns (IsInEffectRange :type Boolean))
  (locals (RetIsInRange :type Boolean :default false))
  (set `local.RetIsInRange` false)
  (for _array_element (`PrimitiveComponent.GetOverlappingActors` (`self.AttackRangeCollisionBox`) "BP_Tower_C")
    (bind _asbp_tower (cast `/Game/BluePrint/Core/Tower/BP_Tower` _array_element))
    (if (== _asbp_tower (`local.TargetTower`))
      (set `local.RetIsInRange` true)
      (break)))
  (return (`local.RetIsInRange`)))

(fn `GetAnEnemyNotEffected`
  (returns (EnemyNotEffected :type "/Game/BluePrint/Core/Character/BP_UnitMaster_Enemy Object Reference"))
  (locals (RetEnemy :type "/Game/BluePrint/Core/Character/BP_UnitMaster_Enemy Object Reference"))
  (for _array_element (`self.UnitEnemyInAttackRange`)
    (if (not (`KismetArrayLibrary.Array_Contains` (`self.EffectedEnemyRecord`) _array_element))
      (set `local.RetEnemy` _array_element)
      (break)))
  (return (`local.RetEnemy`)))

(fn `ModifierAttackRate`
  (params (TimesOfAttackRate :type "Float (double-precision)" :default -999.0))
  (if (and (!= TimesOfAttackRate -999.0) (!= (`self.CurrentAttackRate`) 0.0))
    (`self.SetCurrentAttackRate` (* (`self.CurrentAttackRate`) (`local.TimesOfAttackRate`)))))

(fn `OnEnemyNeedToRemoveFromCombat`
  (params (Enemy :type "/Game/BluePrint/Core/Character/BP_UnitMaster_Enemy Object Reference"))
  (bind _unitenemyinattackrange (`self.UnitEnemyInAttackRange`))
  (if (`KismetArrayLibrary.Array_Contains` _unitenemyinattackrange Enemy)
    (`KismetArrayLibrary.Array_RemoveItem` _unitenemyinattackrange Enemy)
    (`KismetArrayLibrary.Array_RemoveItem` (`self.EffectedEnemyRecord`) Enemy)))

(fn `RefreshEffectRangeOverlappedTowers`
  (`|ExecutionSequence`
    (:`then_0`
      (for _array_element (`self.TowerInEffectRange`)
        (`self.RemoveTowerFromEffectRange` _array_element))
      (`KismetArrayLibrary.Array_Clear` (`self.TowerInEffectRange`)))
    (:`then_1`
      (for _array_element_2 (`PrimitiveComponent.GetOverlappingActors` (`self.AttackRangeCollisionBox`) "BP_Tower_C")
        (bind _asbp_tower (cast `/Game/BluePrint/Core/Tower/BP_Tower` _array_element_2))
        (`self.AddTowerInEffectRange` _asbp_tower)))))

(fn `RemoveBuffOrDebuffFromEffectTower`
  (params (EffectTower :type "/Game/BluePrint/Core/Tower/BP_Tower Object Reference"))
  (switch `/Game/BluePrint/Core/Tower/Utilities/Enum_TowerType` (`/Game/BluePrint/Core/Tower/BP_Tower.TowerType` EffectTower)
    (:`NewEnumerator1`
      (`self.ModifierAttackRate` (/ 2.0 3.0)))))

(fn `RemoveTowerFromEffectRange`
  (params (Tower :type "/Game/BluePrint/Core/Tower/BP_Tower Object Reference"))
  (bind _tower (`local.Tower`))
  (if (`KismetArrayLibrary.Array_Contains` (`self.TowerInEffectRange`) (`local.Tower`))
    (`/Engine/EditorBlueprintResources/StandardMacros.IsValid` _tower
      (:`Is Valid`
        (`KismetArrayLibrary.Array_RemoveItem` (`self.TowerInEffectRange`) _tower)
        (`/Engine/EditorBlueprintResources/StandardMacros.IsValid` self
          (:`Is Valid`
            (`KismetArrayLibrary.Array_RemoveItem` (`/Game/BluePrint/Core/Tower/BP_Tower.ParentTowerOfBuff` _tower) self)
            (`/Engine/EditorBlueprintResources/StandardMacros.IsValid` self
              (:`Is Valid`
                (`self.RemoveBuffOrDebuffFromEffectTower` _tower self)))))))))

(fn `ResetCurrentAttackDamageOrEffectPercent`
  (bind ((`CurrentLevel_11_40A8CAEF4711C73A6E7C9E967904F26E` _currentlevel) (`Level_UpgradeCost_50_6733FF4D4A45895C688BF5BD8A42B08B` _level_upgradecost) (`Level_BaseDamage_33_C856A810464E8553C1BBDDAA2D904B7C` _level_basedamage)) (break `/Game/BluePrint/Core/Tower/Utilities/S_TowerData_Stats_Numerical` (`.Stats_32_516A75554717573F9FE51BA7807FAD22` (break `/Game/BluePrint/Core/Tower/Utilities/S_DefenseTowerData` (`self.TowerData`)))))
  (if (> (`BlueprintMapLibrary.Map_Length` _level_basedamage) 0)
    (bind _keys (`BlueprintMapLibrary.Map_Keys` _level_basedamage))
    (bind _output (`|GetArrayItem` _keys))
    (`self.SetCurrentTowerAttackDamageOrEffectPercent` (`BlueprintMapLibrary.Map_Find` _level_basedamage (`KismetMathLibrary.SelectInt` _output _currentlevel (== _output -999))))
    (else
      (`self.SetCurrentTowerAttackDamageOrEffectPercent` 0.0))))

(fn `ResetCurrentAttackRate`
  (bind ((`CurrentLevel_11_40A8CAEF4711C73A6E7C9E967904F26E` _currentlevel) (`Level_UpgradeCost_50_6733FF4D4A45895C688BF5BD8A42B08B` _level_upgradecost) (`Level_AttackRate_36_3309C992402BFB2DF97CFBBCC4CD3A89` _level_attackrate)) (break `/Game/BluePrint/Core/Tower/Utilities/S_TowerData_Stats_Numerical` (`.Stats_32_516A75554717573F9FE51BA7807FAD22` (break `/Game/BluePrint/Core/Tower/Utilities/S_DefenseTowerData` (`self.TowerData`)))))
  (if (> (`BlueprintMapLibrary.Map_Length` _level_attackrate) 0)
    (bind _keys (`BlueprintMapLibrary.Map_Keys` _level_attackrate))
    (bind _output (`|GetArrayItem` _keys))
    (`self.SetCurrentAttackRate` (`BlueprintMapLibrary.Map_Find` _level_attackrate (`KismetMathLibrary.SelectInt` _output _currentlevel (== _output -999))))
    (else
      (`self.SetCurrentAttackRate` 0.0))))

(fn `SetCurrentAttackRate`
  (params (NewAttackRate :type "Float (double-precision)"))
  (bind _structout (setmembers `/Game/BluePrint/Core/Tower/Utilities/S_TowerData_Stats_Numerical` :`StructRef` (`.Stats_32_516A75554717573F9FE51BA7807FAD22` (break `/Game/BluePrint/Core/Tower/Utilities/S_DefenseTowerData` (`self.TowerData`))) :`Current_AttackRate` NewAttackRate))
  (bind _structout_2 (setmembers `/Game/BluePrint/Core/Tower/Utilities/S_DefenseTowerData` :`StructRef` (`self.TowerData`) :`Stats` _structout))
  (set `self.TowerData` _structout_2)
  (bind _output_get (set `self.CurrentAttackRate` NewAttackRate))
  (`KismetSystemLibrary.PrintString` (`KismetStringLibrary.Concat_StrStr` "Current  Attack  Rate" (`KismetStringLibrary.Conv_DoubleToString` _output_get) (`KismetSystemLibrary.GetDisplayName` self)) true true (struct :`R` 1.0 :`B` 0.039438 :`A` 1.0) 20.0))

(fn `SetCurrentTowerAttackDamageOrEffectPercent`
  (params (CurrentAttackDamageOrEffectPercent :type "Float (single-precision)"))
  (set `self.CurrentAttackDamageOrEffectPercent` CurrentAttackDamageOrEffectPercent))

(fn `SetCurrentTowerLevel`
  (params (NewLevel :type Integer))
  (bind _structout (setmembers `/Game/BluePrint/Core/Tower/Utilities/S_TowerData_Stats_Numerical` :`StructRef` (`.Stats_32_516A75554717573F9FE51BA7807FAD22` (break `/Game/BluePrint/Core/Tower/Utilities/S_DefenseTowerData` (`self.TowerData`))) :`CurrentLevel` (`KismetMathLibrary.Clamp` NewLevel 1 (`.MaxLevel_12_3C3A3FCC4DAA468E51D6F1BC1FD8198C` (break `/Game/BluePrint/Core/Tower/Utilities/S_TowerData_Stats_Numerical` (`.Stats_32_516A75554717573F9FE51BA7807FAD22` (break `/Game/BluePrint/Core/Tower/Utilities/S_DefenseTowerData` (`self.TowerData`))))))))
  (bind _structout_2 (setmembers `/Game/BluePrint/Core/Tower/Utilities/S_DefenseTowerData` :`StructRef` (`self.TowerData`) :`Stats` _structout))
  (set `self.TowerData` _structout_2))

(fn `SetIsHovered`
  (params (Hovered :type Boolean))
  (set `self.IsHovered` Hovered)
  (`self.UpdateVisualIfHoveredOrSelected`))

(fn `SetIsSelected`
  (params (Selected :type Boolean))
  (set `self.IsSelected` Selected)
  (`self.UpdateVisualIfHoveredOrSelected`))

(fn `SetTowerData`
  (params (TowerData :type "/Game/BluePrint/Core/Tower/Utilities/S_DefenseTowerData Structure"))
  (set `self.TowerData` TowerData)
  (`|ExecutionSequence`
    (:`then_0`
      (`self.SetCurrentTowerLevel` 1)
      (`self.ResetCurrentAttackRate`)
      (`self.UpdateVolumeModelBaseOnType`)
      (`self.UpdateAttackRangeBaseToType`)
      (`self.ResetCurrentAttackDamageOrEffectPercent`))
    (:`then_1`
      (if (`self.IsPreviewDisplayTower`)
        (`PrimitiveComponent.SetCollisionEnabled` (`self.AttackRangeCollisionBox`) "NoCollision")
        (bind _returnvalue (`PrimitiveComponent.CreateDynamicMaterialInstance` (`self.SM_TowerVolumeModel`) 0 "/Game/Demo/ArtResource/Material/MI_ColorWithOpacity/MI_ColorWithOpacity_TowerVolume.MI_ColorWithOpacity_TowerVolume" "None"))
        (bind _output_get (set `self.TowerVolumeDynamicMaterial` _returnvalue))
        (`MaterialInstanceDynamic.SetVectorParameterValue` _output_get "Color" (`/Game/BluePrint/Core/Tower/Utilities/BFL_Towers.GetTowerVolumeColorBaseOnType` (`self.TowerType`)))
        (bind _returnvalue_2 (`PrimitiveComponent.CreateDynamicMaterialInstance` (`self.SM_TowerAttackRangeDisplay`) 0 "/Game/BluePrint/Core/Terrain/GridShape/Square/MI_Grid_Flat_PreviewTowerAttackRange.MI_Grid_Flat_PreviewTowerAttackRange" "None"))
        (set `self.TowerAttackRangeDynamicMaterial` _returnvalue_2)
        (else
          (`PrimitiveComponent.SetCollisionEnabled` (`self.AttackRangeCollisionBox`) "QueryOnly")
          (bind _returnvalue_3 (`PrimitiveComponent.CreateDynamicMaterialInstance` (`self.SM_TowerVolumeModel`) 0 "/Game/Demo/ArtResource/Material/MI_Color/MI_Color_TowerVolume.MI_Color_TowerVolume" "None"))
          (bind _output_get_2 (set `self.TowerVolumeDynamicMaterial` _returnvalue_3))
          (`MaterialInstanceDynamic.SetVectorParameterValue` _output_get_2 "Color" (`/Game/BluePrint/Core/Tower/Utilities/BFL_Towers.GetTowerVolumeColorBaseOnType` (`self.TowerType`)))
          (bind _returnvalue_4 (`PrimitiveComponent.CreateDynamicMaterialInstance` (`self.SM_TowerAttackRangeDisplay`) 0 "/Game/BluePrint/Core/Terrain/GridShape/Square/MI_Grid_Flat_TowerAttackRange.MI_Grid_Flat_TowerAttackRange" "None"))
          (set `self.TowerAttackRangeDynamicMaterial` _returnvalue_4))))))

(fn `UpdateAttackRangeBaseToType`
  (locals (DeltaRange :type "Vector Structure") (AttackRangeWithNoChangeBaseOnLevel :type Boolean))
  (bind ((`Level_AttackStartRange_50_19011E784E695B2A3C9F8D88B9C54452` _level_attackstartrange) (`Level_AttackEndRange_51_55D6AF9D4F0B539F72B02884910A2FA3` _level_attackendrange) (`Stats_32_516A75554717573F9FE51BA7807FAD22` _stats)) (break `/Game/BluePrint/Core/Tower/Utilities/S_DefenseTowerData` (`self.TowerData`)))
  (bind ((`Level_AttackStartRange_50_19011E784E695B2A3C9F8D88B9C54452` _level_attackstartrange_2) (`Level_AttackEndRange_51_55D6AF9D4F0B539F72B02884910A2FA3` _level_attackendrange_2) (`AttackDirection_28_DF1C4C004AA4643BC00469BF41B1F5AD` _attackdirection) (`Stats_32_516A75554717573F9FE51BA7807FAD22` _stats_2)) (break `/Game/BluePrint/Core/Tower/Utilities/S_DefenseTowerData` (`self.TowerData`)))
  (bind ((`Level_AttackStartRange_50_19011E784E695B2A3C9F8D88B9C54452` _level_attackstartrange_3) (`Stats_32_516A75554717573F9FE51BA7807FAD22` _stats_3)) (break `/Game/BluePrint/Core/Tower/Utilities/S_DefenseTowerData` (`self.TowerData`)))
  (bind _returnvalue (`KismetMathLibrary.SelectInt` -999 (`.CurrentLevel_11_40A8CAEF4711C73A6E7C9E967904F26E` (break `/Game/BluePrint/Core/Tower/Utilities/S_TowerData_Stats_Numerical` _stats)) (`local.AttackRangeWithNoChangeBaseOnLevel`)))
  (bind _returnvalue_2 (`KismetMathLibrary.SelectInt` -999 (`.CurrentLevel_11_40A8CAEF4711C73A6E7C9E967904F26E` (break `/Game/BluePrint/Core/Tower/Utilities/S_TowerData_Stats_Numerical` _stats_2)) (`local.AttackRangeWithNoChangeBaseOnLevel`)))
  (bind _z (.z (`KismetMathLibrary.Conv_IntVectorToVector` (`BlueprintMapLibrary.Map_Find` _level_attackstartrange_3 (`KismetMathLibrary.SelectInt` -999 (`.CurrentLevel_11_40A8CAEF4711C73A6E7C9E967904F26E` (break `/Game/BluePrint/Core/Tower/Utilities/S_TowerData_Stats_Numerical` _stats_3)) (`local.AttackRangeWithNoChangeBaseOnLevel`))))))
  (bind _z_2 (.z (`KismetMathLibrary.Conv_IntVectorToVector` (`BlueprintMapLibrary.Map_Find` _level_attackstartrange _returnvalue))))
  (bind _returnvalue_3 (`KismetMathLibrary.MakeTransform` (`KismetMathLibrary.MakeVector` 0.0 0.0 (select `bool` (!= _z 0.0) :`true` (* (.z (`self.GridSize`)) _z))) (struct :`Roll` -180.0) (`KismetMathLibrary.MakeVector` (+ (.x (`local.DeltaRange`)) 1.0) (+ (.y (`local.DeltaRange`)) 1.0) (+ (.z (`local.DeltaRange`)) 1.0))))
  (bind _returnvalue_4 (`KismetMathLibrary.MakeTransform` (`KismetMathLibrary.MakeVector` 0.0 0.0 (* (.z (`self.GridSize`)) (+ (/ (- (.z (`KismetMathLibrary.Conv_IntVectorToVector` (`BlueprintMapLibrary.Map_Find` _level_attackendrange _returnvalue))) _z_2) 2.0) _z_2 0.5))) (struct :`Roll` -180.0) (`KismetMathLibrary.MakeVector` (+ (.x (`local.DeltaRange`)) 1.0) (+ (.y (`local.DeltaRange`)) 1.0) (+ (.z (`local.DeltaRange`)) 1.0))))
  (`|ExecutionSequence`
    (:`then_0`
      (bind _keys (`BlueprintMapLibrary.Map_Keys` (`.Level_AttackStartRange_50_19011E784E695B2A3C9F8D88B9C54452` (break `/Game/BluePrint/Core/Tower/Utilities/S_DefenseTowerData` (`self.TowerData`)))))
      (set `local.AttackRangeWithNoChangeBaseOnLevel` (== (`|GetArrayItem` _keys) -999)))
    (:`then_1`
      (set `local.DeltaRange` (- (`KismetMathLibrary.Conv_IntVectorToVector` (`BlueprintMapLibrary.Map_Find` _level_attackendrange_2 _returnvalue_2)) (`KismetMathLibrary.Conv_IntVectorToVector` (`BlueprintMapLibrary.Map_Find` _level_attackstartrange_2 _returnvalue_2))))
      (switch `/Game/BluePrint/Core/Tower/Utilities/Enum_TowerAttackDirection` _attackdirection
        (:`NewEnumerator0`
          (`SceneComponent.K2_SetRelativeTransform` (`self.SM_TowerAttackRangeDisplay`) _returnvalue_3 false false)
          (`SceneComponent.K2_SetRelativeTransform` (`self.AttackRangeCollisionBox`) _returnvalue_4 false false))
        (:`NewEnumerator2`
          (`SceneComponent.K2_SetRelativeTransform` (`self.SM_TowerAttackRangeDisplay`) _returnvalue_3 false false)
          (`SceneComponent.K2_SetRelativeTransform` (`self.AttackRangeCollisionBox`) _returnvalue_4 false false))))))

(fn `UpdateVisualIfHoveredOrSelected`
  (`MeshComponent.SetVectorParameterValueOnMaterials` (`self.SM_TowerVolumeModel`) "ColorMultiply" (`KismetMathLibrary.Conv_LinearColorToVector` (* (* (select `bool` (`self.IsSelected`) :`false` (struct :`R` 1.0 :`G` 1.0 :`B` 1.0 :`A` 1.0) :`true` (struct :`G` 1.0 :`B` 0.754485 :`A` 1.0) :!type "LinearColor Structure") (select `bool` (`self.IsHovered`) :`false` 1.0 :`true` 2.5 :!type "Float (single-precision)")) (select `bool` (`self.IsSelected`) :`false` 1.0 :`true` 2.5 :!type "Float (single-precision)"))))
  (`SceneComponent.SetVisibility` (`self.SM_TowerAttackRangeDisplay`) (or (`self.IsHovered`) (`self.IsSelected`)) false))

(fn `UpdateVolumeModelBaseOnType`
  (bind (_x _y _z) (break `IntVector` (`.VolumeOfConstruction_17_4EAEDD0C451DF68CF80791B0A4092882` (break `/Game/BluePrint/Core/Tower/Utilities/S_DefenseTowerData` (`self.TowerData`)))))
  (`SceneComponent.SetRelativeScale3D` (`self.SM_TowerVolumeModel`) (`KismetMathLibrary.MakeVector` (`KismetMathLibrary.Conv_IntToDouble` _x) (`KismetMathLibrary.Conv_IntToDouble` _y) (select `bool` (== _z -1) :`false` (`KismetMathLibrary.Conv_IntToDouble` _z) :`true` 0.3))))

(fn `UserConstructionScript`
  (`self.SetTowerData` (`/Game/BluePrint/Core/Tower/Utilities/BFL_Towers.GetDefaultTowerDataBaseOnTowerType` (`self.TowerType`))))