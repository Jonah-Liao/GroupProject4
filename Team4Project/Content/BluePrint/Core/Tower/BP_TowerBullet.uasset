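; BP_TowerBullet is a tower projectile that homes in on a target enemy and damages it.
; From BeginPlay, a timeline lerps the bullet from its current location toward the moving target each update, destroying it when the target is invalid or the timeline finishes.
; Overlapping any enemy unit makes that enemy the target, applies BulletDamage through ModiferCurrentHp, and destroys the bullet after a short delay.
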(event `self.ReceiveBeginPlay`
  (`self.ShootToEnemy`))

(event `ShootToEnemy`
  (bind (_direction _bulletlocation) (`Timeline|Timeline` :!via `PlayFromStart`)
    (:`Update`
      (`/Engine/EditorBlueprintResources/StandardMacros.IsValid` (`self.TargetEnemy`)
        (:`Is Valid`
          (`self.K2_SetActorLocation` (`KismetMathLibrary.VLerp` (`self.K2_GetActorLocation`) (`self.K2_GetActorLocation` (`self.TargetEnemy`)) _bulletlocation)))
        (:`Is Not Valid`
          (`self.K2_DestroyActor` :!label _label))))
    (:`Finished`
      (`KismetSystemLibrary.PrintString` "TowerBulletHitEnemy")
      (goto _label))))

(event `self.Sphere_BulletCollision.OnComponentBeginOverlap`
  (params (OverlappedComponent :type "PrimitiveComponent Object Reference") (OtherActor :type "Actor Object Reference") (OtherComp :type "PrimitiveComponent Object Reference") (OtherBodyIndex :type Integer) (bFromSweep :type Boolean) (SweepResult :type "HitResult Structure (by ref)"))
  (bind _asbp_unit_master_enemy (cast `/Game/BluePrint/Core/Character/BP_UnitMaster_Enemy` OtherActor))
  (if (== _asbp_unit_master_enemy (`self.TargetEnemy`))
    (`KismetSystemLibrary.PrintString` (`KismetStringLibrary.Concat_StrStr` "HitTarget" (`KismetSystemLibrary.GetDisplayName` (`self.TargetEnemy`))))
    (else
      (set `self.TargetEnemy` _asbp_unit_master_enemy)))
  (`/Game/BluePrint/Core/Character/BP_UnitMaster_Enemy.ModiferCurrentHp` (`self.TargetEnemy`) (`self.BulletDamage`))
  (`KismetSystemLibrary.Delay` 0.2)
  (`self.K2_DestroyActor`))

(fn `UserConstructionScript`)