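; Enemy spawn point actor that spawns a wave of BP_UnitMaster_Enemy units at its location and gives each a waypoint path.
; SpawnWaveOfEnemy waits an initial delay, then walks a map of enemy types to counts, spawning each unit with a delay between spawns.
; Manual-advance loop macros allow the delays inside the nested loops, and a busy flag blocks overlapping waves.
; Dispatchers announce each new enemy and when the line finishes spawning.
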(event `self.ReceiveBeginPlay`)

(event `SpawnWaveOfEnemy`
  (params (DelayBeforeStart :type "Float (double-precision)") (EnemyPath :type "Array of /Game/BluePrint/Core/WayPoint/BP_WayPoint Object Reference") (EnemyTypeAndNum :type "Map of /Game/BluePrint/Core/Character/Utilities_Enemy/Enum_EnemyType Enum to Integer") (DelayBetweenEachEnemySpawn :type "Float (double-precision)" :default 0.5))
  (if (not (`self.IsSpawningEnemy`))
    (set `self.IsSpawningEnemy` true)
    (`KismetSystemLibrary.Delay` DelayBeforeStart)
    (bind _keys (`BlueprintMapLibrary.Map_Keys` EnemyTypeAndNum))
    (bind _array_element (`/Game/BluePrint/Core/Utilities/StandardMacros_Manual.ForEachLoopManual` _keys :!label _label)
      (:`LoopBody`
        (`/Game/BluePrint/Core/Utilities/StandardMacros_Manual.ForLoopManual` 0 (- (`BlueprintMapLibrary.Map_Find` EnemyTypeAndNum _array_element) 1) :!label _label_2
          (:`LoopBody`
            (bind _returnvalue (`|SpawnActorFromClass` "/Game/BluePrint/Core/Character/BP_UnitMaster_Enemy.BP_UnitMaster_Enemy_C" (`KismetMathLibrary.MakeTransform` (`self.K2_GetActorLocation`)) "AdjustIfPossibleButAlwaysSpawn" "MultiplyWithRoot" null EnemyPath true _array_element null))
            (`self.OnNewEnemySpawned` _returnvalue)
            (`KismetSystemLibrary.Delay` DelayBetweenEachEnemySpawn)
            (goto _label_2 :!via `NextLoop`))
          (:`Completed`
            (goto _label :!via `NextLoop`))))
      (:`Completed`
        (`self.OnCurrentEnemyLineFinishedSpawning`)
        (set `self.IsSpawningEnemy` false)))))

(fn `UserConstructionScript`)