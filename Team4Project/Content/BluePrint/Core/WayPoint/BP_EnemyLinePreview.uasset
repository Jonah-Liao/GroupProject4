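; BP_EnemyLinePreview is a waypoint-related actor that shows a preview line for enemies using a stretched cube.
; On BeginPlay it scales CubeLinePreview to a thin bar, setting Z to the StartLocation–EndLocation distance divided by the cube's Z size.
; It only sets scale, not position or rotation.
; A copy of this scaling sits unconnected in the Construction Script, so it never runs there.
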(event `self.ReceiveBeginPlay`
  (`SceneComponent.SetRelativeScale3D` (`self.Cube_LinePreview`) (`KismetMathLibrary.MakeVector` 0.3 0.3 (/ (`KismetMathLibrary.Vector_Distance` (`self.EndLocation`) (`self.StartLocation`)) (.z (`self.CubeSize`))))))

(fn `UserConstructionScript`)