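; BP_CombatSystem tracks towers placed in combat and keeps them synced with the terrain's tile grid.
; Adding, moving or removing a tower rewrites the per-side tower entries in Terrain tile data.
; Each tower is positioned at the center of its tile group, offset and rotated for its tile side and rotate flag, or sent far off-map without valid tiles.
; Terrain generation and tile update events re-apply placement or destroy towers on unbuildable tiles.
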(event `self.ReceiveBeginPlay`
  (bind _terrain (`self.Terrain`))
  (add `/Game/BluePrint/Core/Terrain/BP_Terrain.OnTerrainGenerated` _terrain (`|CreateDelegate` :!event `OnTerrainGenerated`))
  (add `/Game/BluePrint/Core/Terrain/BP_Terrain.OnTileDataUpdated` _terrain (`|CreateDelegate` :!event `OnTileDataUpdated`)))

(fn `AddTowerInCombat`
  (params (Tower :type "/Game/BluePrint/Core/Tower/BP_Tower Object Reference") (TerrainIndexesAndSideIndexes :type "Map of IntVector Structure to Integer") (IsRotate :type Boolean))
  (`KismetArrayLibrary.Array_Add` (`self.TowerInCombat`) (`local.Tower`))
  (`self.SetTowerTerrainIndexesAndSideIndexesInMap` (`local.Tower`) (`local.TerrainIndexesAndSideIndexes`) IsRotate))

(fn `CalculateTowerTargetLocAndRotFromIndexGroupAndSideIndexGroup`
  (params (TargetTerrainIndexesAndTileSideIndexes :type "Map of IntVector Structure to Integer") (IsRotate :type Boolean))
  (returns (TargetLocation :type "Vector Structure") (TargetRotation :type "Rotator Structure"))
  (locals (LeftBottomTerrainIndex :type "IntVector Structure" :default (struct)) (RightTopTerrainIndex :type "IntVector Structure" :default (struct)) (TargetCenterLoc :type "Vector Structure") (TargetCenterRot :type "Rotator Structure" :default (struct)))
  (bind _isrotate (`local.IsRotate`))
  (bind (_x _y _z) (break `IntVector` (`local.LeftBottomTerrainIndex`)))
  (bind (_x_2 _y_2 _z_2) (break `IntVector` (`local.RightTopTerrainIndex`)))
  (bind _location (.location (`.Center_20_A6FFDF2D4282E067847953B7B01B67F3` (break `/Game/BluePrint/Core/Terrain/Utilities/S_SidesOfGridTransform` (`.TransformOfAllSide_17_7BB94EF04670051629E034A2A56399CD` (break `/Game/BluePrint/Core/Terrain/Utilities/S_TileData` (`BlueprintMapLibrary.Map_Find` (`/Game/BluePrint/Core/Terrain/BP_Terrain.TerrainGridTiles` (`self.Terrain`)) (`local.LeftBottomTerrainIndex`))))))))
  (`|ExecutionSequence`
    (:`then_0`
      (set `local.LeftBottomTerrainIndex` (make `IntVector` 999999 999999 999999))
      (set `local.RightTopTerrainIndex` (make `IntVector` -999999 -999999 -999999)))
    (:`then_1`
      (bind _keys (`BlueprintMapLibrary.Map_Keys` (`local.TargetTerrainIndexesAndTileSideIndexes`)))
      (for _array_element _keys
        (bind (_x_3 _y_3 _z_3) (break `IntVector` _array_element))
        (set `local.LeftBottomTerrainIndex` (make `IntVector` (`KismetMathLibrary.Min` _x_3 _x) (`KismetMathLibrary.Min` _y_3 _y) (`KismetMathLibrary.Min` _z_3 _z)))))
    (:`then_2`
      (bind _keys_2 (`BlueprintMapLibrary.Map_Keys` (`local.TargetTerrainIndexesAndTileSideIndexes`)))
      (for _array_element_2 _keys_2
        (bind (_x_4 _y_4 _z_4) (break `IntVector` _array_element_2))
        (set `local.RightTopTerrainIndex` (make `IntVector` (`KismetMathLibrary.Max` _x_4 _x_2) (`KismetMathLibrary.Max` _y_4 _y_2) (`KismetMathLibrary.Max` _z_4 _z_2)))))
    (:`then_3`
      (set `local.TargetCenterLoc` (+ (/ (- (.location (`.Center_20_A6FFDF2D4282E067847953B7B01B67F3` (break `/Game/BluePrint/Core/Terrain/Utilities/S_SidesOfGridTransform` (`.TransformOfAllSide_17_7BB94EF04670051629E034A2A56399CD` (break `/Game/BluePrint/Core/Terrain/Utilities/S_TileData` (`BlueprintMapLibrary.Map_Find` (`/Game/BluePrint/Core/Terrain/BP_Terrain.TerrainGridTiles` (`self.Terrain`)) (`local.RightTopTerrainIndex`))))))) _location) 2.0) _location))
      (bind _values (`BlueprintMapLibrary.Map_Values` (`local.TargetTerrainIndexesAndTileSideIndexes`)))
      (switch `int` (`|GetArrayItem` _values) ; 0 Top\n1 Bottom\n2 Front\n3 Back\n4 Left\n5 Right
        (:`0`
          (set `local.TargetCenterLoc` (`KismetMathLibrary.MakeVector` (.x (`local.TargetCenterLoc`)) (.y (`local.TargetCenterLoc`)) (+ (.z (`local.TargetCenterLoc`)) (/ (.z (`/Game/BluePrint/Core/Terrain/BP_Terrain.TerrainGridSize` (`self.Terrain`))) 2.0)))))
        (:`1`
          (set `local.TargetCenterLoc` (`KismetMathLibrary.MakeVector` (.x (`local.TargetCenterLoc`)) (.y (`local.TargetCenterLoc`)) (- (.z (`local.TargetCenterLoc`)) (/ (.z (`/Game/BluePrint/Core/Terrain/BP_Terrain.TerrainGridSize` (`self.Terrain`))) 2.0)))))
        (:`2`
          (set `local.TargetCenterLoc` (`KismetMathLibrary.MakeVector` (+ (.x (`local.TargetCenterLoc`)) (/ (.z (`/Game/BluePrint/Core/Terrain/BP_Terrain.TerrainGridSize` (`self.Terrain`))) 2.0)) (.y (`local.TargetCenterLoc`)) (.z (`local.TargetCenterLoc`)))))
        (:`3`
          (set `local.TargetCenterLoc` (`KismetMathLibrary.MakeVector` (- (.x (`local.TargetCenterLoc`)) (/ (.z (`/Game/BluePrint/Core/Terrain/BP_Terrain.TerrainGridSize` (`self.Terrain`))) 2.0)) (.y (`local.TargetCenterLoc`)) (.z (`local.TargetCenterLoc`)))))
        (:`4`
          (set `local.TargetCenterLoc` (`KismetMathLibrary.MakeVector` (.x (`local.TargetCenterLoc`)) (- (.y (`local.TargetCenterLoc`)) (/ (.z (`/Game/BluePrint/Core/Terrain/BP_Terrain.TerrainGridSize` (`self.Terrain`))) 2.0)) (.z (`local.TargetCenterLoc`)))))
        (:`5`
          (set `local.TargetCenterLoc` (`KismetMathLibrary.MakeVector` (.x (`local.TargetCenterLoc`)) (+ (.y (`local.TargetCenterLoc`)) (/ (.z (`/Game/BluePrint/Core/Terrain/BP_Terrain.TerrainGridSize` (`self.Terrain`))) 2.0)) (.z (`local.TargetCenterLoc`)))))))
    (:`then_4`
      (bind _values_2 (`BlueprintMapLibrary.Map_Values` (`local.TargetTerrainIndexesAndTileSideIndexes`)))
      (set `local.TargetCenterRot` (select `int` (`|GetArrayItem` _values_2) :`0` (select `bool` _isrotate :`false` (struct :`Yaw` 90.0) :!type "Rotator Structure") :`1` (select `bool` _isrotate :`false` (struct :`Yaw` 90.0 :`Roll` 180.0) :`true` (struct :`Roll` 180.0) :!type "Rotator Structure") :`2` (select `bool` _isrotate :`false` (struct :`Pitch` -90.0) :`true` (struct :`Yaw` -90.0 :`Roll` 90.0) :!type "Rotator Structure") :`3` (select `bool` _isrotate :`false` (struct :`Pitch` 90.0) :`true` (struct :`Yaw` 90.0 :`Roll` 90.0) :!type "Rotator Structure") :`4` (select `bool` _isrotate :`false` (struct :`Pitch` 90.0 :`Roll` -90.0) :`true` (struct :`Roll` -90.0) :!type "Rotator Structure") :`5` (select `bool` _isrotate :`false` (struct :`Pitch` 90.0 :`Roll` 90.0) :`true` (struct :`Roll` 90.0) :!type "Rotator Structure"))))
    (:`then_5`
      (return (`local.TargetCenterLoc`) (`local.TargetCenterRot`)))))

(fn `OnTerrainGenerated`
  (locals (TempTowerInCombat :type "Array of /Game/BluePrint/Core/Tower/BP_Tower Object Reference") (T :type "/Game/BluePrint/Core/Tower/BP_Tower Object Reference"))
  (bind _t (`local.T`))
  (bind _output_get (set `local.TempTowerInCombat` (`self.TowerInCombat`)))
  (for _array_element _output_get
    (set `local.T` _array_element)
    (bind _keys (`BlueprintMapLibrary.Map_Keys` (`/Game/BluePrint/Core/Tower/BP_Tower.TerrainIndexesAndSideIndexes` (`local.T`))))
    (if (`/Game/BluePrint/Core/Terrain/BP_Terrain.IsTerrainIndexGroupAllTowerBuildable` (`self.Terrain`) _keys)
      (`self.SetTowerTerrainIndexesAndSideIndexesInMap` (`local.T`) (`/Game/BluePrint/Core/Tower/BP_Tower.TerrainIndexesAndSideIndexes` _t) (`/Game/BluePrint/Core/Tower/BP_Tower.IsCurrentTowerRotate` _t) true)
      (else
        (`self.RemoveTowerInCombat` (`local.T`))))))

(fn `OnTileDataUpdated`
  (params (TerrainIndex :type "IntVector Structure"))
  (locals (TempTowerInCombat :type "Array of /Game/BluePrint/Core/Tower/BP_Tower Object Reference") (T :type "/Game/BluePrint/Core/Tower/BP_Tower Object Reference"))
  (bind _t (`local.T`))
  (bind _output_get (set `local.TempTowerInCombat` (`self.TowerInCombat`)))
  (for _array_element _output_get
    (set `local.T` _array_element)
    (bind _keys (`BlueprintMapLibrary.Map_Keys` (`/Game/BluePrint/Core/Tower/BP_Tower.TerrainIndexesAndSideIndexes` (`local.T`))))
    (if (`KismetArrayLibrary.Array_Contains` _keys (`local.TerrainIndex`))
      (if (`/Game/BluePrint/Core/Terrain/BP_Terrain.IsTerrainIndexGroupAllTowerBuildable` (`self.Terrain`) _keys)
        (`self.SetTowerTerrainIndexesAndSideIndexesInMap` (`local.T`) (`/Game/BluePrint/Core/Tower/BP_Tower.TerrainIndexesAndSideIndexes` _t) (`/Game/BluePrint/Core/Tower/BP_Tower.IsCurrentTowerRotate` _t))
        (break)
        (else
          (`self.RemoveTowerInCombat` (`local.T`))
          (break))))))

(fn `RemoveTowerInCombat`
  (params (Tower :type "/Game/BluePrint/Core/Tower/BP_Tower Object Reference") (IsDestroyTower :type Boolean :default true))
  (`KismetArrayLibrary.Array_RemoveItem` (`self.TowerInCombat`) (`local.Tower`))
  (`self.SetTowerTerrainIndexesAndSideIndexesInMap` (`local.Tower`) (`|MakeMap`))
  (if IsDestroyTower
    (`self.K2_DestroyActor` (`local.Tower`))))

(fn `SetTowerTerrainIndexesAndSideIndexesInMap`
  (params (Tower :type "/Game/BluePrint/Core/Tower/BP_Tower Object Reference") (NewTerrainIndexesAndSideIndexes :type "Map of IntVector Structure to Integer") (IsRotateTower :type Boolean) (Force :type Boolean))
  (locals (TempTerrainIndexData :type "/Game/BluePrint/Core/Terrain/Utilities/S_TileData Structure") (TempTowerOnSideTileIndex :type "Map of Integer to /Game/BluePrint/Core/Tower/BP_Tower Object Reference") (TempTerrainI :type "IntVector Structure"))
  (bind _tower (`local.Tower`))
  (bind _tower_2 (`local.Tower`))
  (bind _newterrainindexesandsideindexes (`local.NewTerrainIndexesAndSideIndexes`))
  (bind _terrainindexesandsideindexes (`/Game/BluePrint/Core/Tower/BP_Tower.TerrainIndexesAndSideIndexes` (`local.Tower`)))
  (`|ExecutionSequence`
    (:`then_0`
      (if (> (`BlueprintMapLibrary.Map_Length` (`/Game/BluePrint/Core/Tower/BP_Tower.TerrainIndexesAndSideIndexes` (`local.Tower`))) 0)
        (if (> (`BlueprintMapLibrary.Map_Length` (`local.NewTerrainIndexesAndSideIndexes`)) 0)
          (bind _keys (`BlueprintMapLibrary.Map_Keys` _terrainindexesandsideindexes))
          (bind _keys_2 (`BlueprintMapLibrary.Map_Keys` _newterrainindexesandsideindexes))
          (bind _values (`BlueprintMapLibrary.Map_Values` _terrainindexesandsideindexes))
          (bind _values_2 (`BlueprintMapLibrary.Map_Values` _newterrainindexesandsideindexes))
          (if (or (not (`KismetArrayLibrary.Array_Identical` _keys_2 _keys)) (!= (`|GetArrayItem` _values_2) (`|GetArrayItem` _values)) (`local.Force`))
            (`|ExecutionSequence` :!label _label
              (:`then_0`
                (bind _keys_3 (`BlueprintMapLibrary.Map_Keys` (`/Game/BluePrint/Core/Tower/BP_Tower.TerrainIndexesAndSideIndexes` (`local.Tower`))))
                (for _array_element _keys_3
                  (set `local.TempTerrainI` _array_element)
                  (bind _output_get (set `local.TempTerrainIndexData` (`BlueprintMapLibrary.Map_Find` (`/Game/BluePrint/Core/Terrain/BP_Terrain.TerrainGridTiles` (`self.Terrain`)) _array_element)))
                  (bind _output_get_2 (set `local.TempTowerOnSideTileIndex` (`.TowerOnSideTile_28_CD3C8427467A2C9D9223D5932B9C9EDF` (break `/Game/BluePrint/Core/Terrain/Utilities/S_TileData` _output_get))))
                  (bind _values_3 (`BlueprintMapLibrary.Map_Values` _output_get_2))
                  (if (`KismetArrayLibrary.Array_Contains` _values_3 _tower)
                    (bind _keys_4 (`BlueprintMapLibrary.Map_Keys` (`local.TempTowerOnSideTileIndex`)))
                    (`BlueprintMapLibrary.Map_Remove` (`local.TempTowerOnSideTileIndex`) (`|GetArrayItem` _keys_4 (`KismetArrayLibrary.Array_Find` _values_3 _tower)))
                    (bind _structout (setmembers `/Game/BluePrint/Core/Terrain/Utilities/S_TileData` :`StructRef` (`local.TempTerrainIndexData`) :`TowerOnSideTile` (`local.TempTowerOnSideTileIndex`)))
                    (set `local.TempTerrainIndexData` _structout)
                    (`BlueprintMapLibrary.Map_Add` (`/Game/BluePrint/Core/Terrain/BP_Terrain.TerrainGridTiles` (`self.Terrain`)) (`local.TempTerrainI`) (`local.TempTerrainIndexData`))))
                (set `/Game/BluePrint/Core/Tower/BP_Tower.TerrainIndexesAndSideIndexes` (`|MakeMap`) (`local.Tower`)))
              (:`then_1`
                (set `/Game/BluePrint/Core/Tower/BP_Tower.TerrainIndexesAndSideIndexes` (`local.NewTerrainIndexesAndSideIndexes`) (`local.Tower`))
                (if (> (`BlueprintMapLibrary.Map_Length` (`/Game/BluePrint/Core/Tower/BP_Tower.TerrainIndexesAndSideIndexes` (`local.Tower`))) 0)
                  (bind _keys_5 (`BlueprintMapLibrary.Map_Keys` (`/Game/BluePrint/Core/Tower/BP_Tower.TerrainIndexesAndSideIndexes` (`local.Tower`))))
                  (for _array_element_2 _keys_5
                    (set `local.TempTerrainI` _array_element_2)
                    (bind _output_get_3 (set `local.TempTerrainIndexData` (`BlueprintMapLibrary.Map_Find` (`/Game/BluePrint/Core/Terrain/BP_Terrain.TerrainGridTiles` (`self.Terrain`)) _array_element_2)))
                    (set `local.TempTowerOnSideTileIndex` (`.TowerOnSideTile_28_CD3C8427467A2C9D9223D5932B9C9EDF` (break `/Game/BluePrint/Core/Terrain/Utilities/S_TileData` _output_get_3)))
                    (bind _values_4 (`BlueprintMapLibrary.Map_Values` (`local.NewTerrainIndexesAndSideIndexes`)))
                    (`BlueprintMapLibrary.Map_Add` (`local.TempTowerOnSideTileIndex`) (`|GetArrayItem` _values_4) (`local.Tower`))
                    (bind _structout_2 (setmembers `/Game/BluePrint/Core/Terrain/Utilities/S_TileData` :`StructRef` (`local.TempTerrainIndexData`) :`TowerOnSideTile` (`local.TempTowerOnSideTileIndex`)))
                    (set `local.TempTerrainIndexData` _structout_2)
                    (`BlueprintMapLibrary.Map_Add` (`/Game/BluePrint/Core/Terrain/BP_Terrain.TerrainGridTiles` (`self.Terrain`)) (`local.TempTerrainI`) (`local.TempTerrainIndexData`)))))))
          (else
            (goto _label)))
        (else
          (goto _label))))
    (:`then_1`
      (if (> (`BlueprintMapLibrary.Map_Length` (`local.NewTerrainIndexesAndSideIndexes`)) 0)
        (bind _keys_6 (`BlueprintMapLibrary.Map_Keys` (`local.NewTerrainIndexesAndSideIndexes`)))
        (if (`/Game/BluePrint/Core/Terrain/BP_Terrain.IsTerrainIndexGroupValid` (`self.Terrain`) _keys_6)
          (bind (_targetlocation _targetrotation) (`self.CalculateTowerTargetLocAndRotFromIndexGroupAndSideIndexGroup` (`local.NewTerrainIndexesAndSideIndexes`) (`local.IsRotateTower`)))
          (`self.K2_SetActorLocationAndRotation` _tower_2 _targetlocation _targetrotation false false)
          (set `/Game/BluePrint/Core/Tower/BP_Tower.IsCurrentTowerRotate` (`local.IsRotateTower`) _tower_2)
          (else
            (`self.K2_SetActorLocationAndRotation` :`self` (`local.Tower`) :`NewLocation` (-999999.0 -999999.0 -999999.0) :!label _label_2)))
        (else
          (goto _label_2))))))

(fn `UserConstructionScript`)