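; Player-controlled character base for a combat game with tower building, translating Enhanced Input into movement and gameplay actions.
; Camera-relative movement, look and jump are locked during combat finishing.
; Slot selection, tower shortcuts, clicks, break skipping, pausing and pawn possession switching work through PlayerAction, with left click repeating only in shooting state.
; It also line-traces terrain from the camera and returns the player to the start location on touching death areas.
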(event `self.ReceiveBeginPlay`
  (bind _returnvalue (pcsubsystem `EnhancedInputLocalPlayerSubsystem` (`GameplayStatics.GetPlayerController` 0)))
  (`parent.ReceiveBeginPlay`)
  (`|ExecutionSequence`
    (:`then_0`
      (set `self.StartLocation` (`self.K2_GetActorLocation`)))
    (:`then_1`
      ;[0 0 0 0.5] 加载玩家输入功能
      (`/Engine/EditorBlueprintResources/StandardMacros.IsValid` _returnvalue
        (:`Is Valid`
          (`EnhancedInputSubsystemInterface.AddMappingContext` _returnvalue "/Game/BluePrint/Core/Player/Input/IMC_PlayerAction.IMC_PlayerAction" 0 (struct)))))))

(event `EnhancedInput|/Game/BluePrint/Core/Player/Input/IA_LookAround`
  (params (ActionValue :type "Vector2D Structure") (ElapsedSeconds :type "Float (double-precision)") (TriggeredSeconds :type "Float (double-precision)") (InputAction :type "InputAction Object Reference" :default "/Game/BluePrint/Core/Player/Input/IA_LookAround.IA_LookAround"))
  ;[0 0 0 0.5] 鼠标移动的时候视角跟着移动
  (:`Triggered`
    (if (not (`/Game/BluePrint/Core/Combat/BP_CombatSystem.IsFinishingCombat` (`/Game/BluePrint/Core/Player/BP_PlayerAction.CombatSystem` (`self.PlayerAction`))))
      (`self.AddControllerYawInput` ActionValue_X) ; 左右看
      (`self.AddControllerPitchInput` ActionValue_Y) ; 上下看
    )))

(event `EnhancedInput|/Game/BluePrint/Core/Player/Input/IA_PlayerMovement`
  (params (ActionValue :type "Vector2D Structure") (ElapsedSeconds :type "Float (double-precision)") (TriggeredSeconds :type "Float (double-precision)") (InputAction :type "InputAction Object Reference" :default "/Game/BluePrint/Core/Player/Input/IA_PlayerMovement.IA_PlayerMovement"))
  (bind (_returnvalue_roll _returnvalue_pitch _returnvalue_yaw) (`KismetMathLibrary.BreakRotator` (`self.GetControlRotation`)))
  (bind (_returnvalue_roll_2 _returnvalue_pitch_2 _returnvalue_yaw_2) (`KismetMathLibrary.BreakRotator` (`self.GetControlRotation`)))
  ;[0 0 0 0.5] 移动的时候身体转向摄像头面对的方向
  (:`Triggered`
    (if (not (`/Game/BluePrint/Core/Combat/BP_CombatSystem.IsFinishingCombat` (`/Game/BluePrint/Core/Player/BP_PlayerAction.CombatSystem` (`self.PlayerAction`))))
      (`self.AddMovementInput` (`KismetMathLibrary.GetForwardVector` (`KismetMathLibrary.MakeRotator` 0.0 0.0 _returnvalue_yaw)) ActionValue_X)
      (`self.AddMovementInput` (`KismetMathLibrary.GetRightVector` (`KismetMathLibrary.MakeRotator` 0.0 0.0 _returnvalue_yaw_2)) ActionValue_Y))))

(event `EnhancedInput|/Game/BluePrint/Core/Player/Input/IA_ActiveJump`
  (params (ActionValue :type Boolean) (ElapsedSeconds :type "Float (double-precision)") (TriggeredSeconds :type "Float (double-precision)") (InputAction :type "InputAction Object Reference" :default "/Game/BluePrint/Core/Player/Input/IA_ActiveJump.IA_ActiveJump"))
  (:`Started`
    (if (not (`/Game/BluePrint/Core/Combat/BP_CombatSystem.IsFinishingCombat` (`/Game/BluePrint/Core/Player/BP_PlayerAction.CombatSystem` (`self.PlayerAction`))))
      (`self.Jump`)))
  (:`Completed`
    (`self.StopJumping`)))

(event `EnhancedInput|/Game/BluePrint/Core/Player/Input/IA_ControllerPossessSwitch`
  (params (ActionValue :type Boolean) (ElapsedSeconds :type "Float (double-precision)") (TriggeredSeconds :type "Float (double-precision)") (InputAction :type "InputAction Object Reference" :default "/Game/BluePrint/Core/Player/Input/IA_ControllerPossessSwitch.IA_ControllerPossessSwitch"))
  (bind _playeraction (`self.PlayerAction`))
  (bind _pawn (`self.Pawn`))
  (bind _controllercurrentstate (`/Game/BluePrint/Core/Player/BP_PlayerAction.ControllerCurrentState` _playeraction))
  ; Comment
  (:`Triggered`
    (if ActionValue
      (if (`self.IsAbleToSwitchPossess`)
        (`/Engine/EditorBlueprintResources/StandardMacros.IsValid` _playeraction
          (:`Is Valid`
            (if (or (`|EnumEquality` _controllercurrentstate "NewEnumerator1") (`|EnumEquality` _controllercurrentstate "NewEnumerator2"))
              (set `self.IsAbleToSwitchPossess` false)
              (`/Engine/EditorBlueprintResources/StandardMacros.IsValid` _pawn
                (:`Is Valid`
                  (`Controller.Possess` (`GameplayStatics.GetPlayerController` 0) _pawn)
                  (`self.OnControllerSwitchToPawn`))))))))))

(event `EnhancedInput|/Game/BluePrint/Core/Player/Input/IA_PauseGame`
  (params (ActionValue :type Boolean) (ElapsedSeconds :type "Float (double-precision)") (TriggeredSeconds :type "Float (double-precision)") (InputAction :type "InputAction Object Reference" :default "/Game/BluePrint/Core/Player/Input/IA_PauseGame.IA_PauseGame"))
  (bind _playeraction (`self.PlayerAction`))
  (:`Triggered`
    (if ActionValue
      (if (not (`/Game/BluePrint/Core/Player/BP_PlayerAction.IsGamePause` _playeraction))
        (set `/Game/BluePrint/Core/Player/BP_PlayerAction.IsGamePause` true _playeraction)
        (`GameplayStatics.SetGamePaused` true)
        (`KismetSystemLibrary.PrintString` "PauseGame")
        (`self.OnGamePaused`)))))

(event `EnhancedInput|/Game/BluePrint/Core/Player/Input/IA_SlotSwitch`
  (params (ActionValue :type "Float (double-precision)") (ElapsedSeconds :type "Float (double-precision)") (TriggeredSeconds :type "Float (double-precision)") (InputAction :type "InputAction Object Reference" :default "/Game/BluePrint/Core/Player/Input/IA_SlotSwitch.IA_SlotSwitch"))
  (bind _playeraction (`self.PlayerAction`))
  (bind _playeraction_2 (`self.PlayerAction`))
  (bind _playeraction_3 (`self.PlayerAction`))
  (:`Triggered`
    (if (!= ActionValue 0.0)
      (if (> ActionValue 0.0)
        (set `/Game/BluePrint/Core/Player/BP_PlayerAction.CurrentSlotIndex` (- (`/Game/BluePrint/Core/Player/BP_PlayerAction.CurrentSlotIndex` _playeraction_2) 1) _playeraction_2)
        (else
          (set `/Game/BluePrint/Core/Player/BP_PlayerAction.CurrentSlotIndex` (+ (`/Game/BluePrint/Core/Player/BP_PlayerAction.CurrentSlotIndex` _playeraction_3) 1) _playeraction_3)))
      (`/Game/BluePrint/Core/Player/BP_PlayerAction.SetCurrentSelectedSlotOnWidget` _playeraction (`/Game/BluePrint/Core/Player/BP_PlayerAction.CurrentSlotIndex` _playeraction)))))

(event `EnhancedInput|/Game/BluePrint/Core/Player/Input/IA_RemoveTower`
  (params (ActionValue :type Boolean) (ElapsedSeconds :type "Float (double-precision)") (TriggeredSeconds :type "Float (double-precision)") (InputAction :type "InputAction Object Reference" :default "/Game/BluePrint/Core/Player/Input/IA_RemoveTower.IA_RemoveTower"))
  (bind _playeraction (`self.PlayerAction`))
  (bind _combatsystem (`/Game/BluePrint/Core/Player/BP_PlayerAction.CombatSystem` _playeraction))
  (bind _combatdebugwidget (`/Game/BluePrint/Core/Combat/BP_CombatSystem.CombatDebugWidget` _combatsystem))
  (:`Triggered`
    (`/Engine/EditorBlueprintResources/StandardMacros.IsValid` _combatdebugwidget
      (:`Is Valid`
        (bind _output_get (set `/Game/BluePrint/Core/Player/BP_PlayerAction.CurrentSlotIndex` (- (`PanelWidget.GetChildrenCount` (`/Game/BluePrint/Core/Combat/DebugWidget/WBP_VerticalSlot.vBox_SlotGroup` (`/Game/BluePrint/Core/Combat/DebugWidget/WBP_DebugCombatScreen.WBP_VerticalSlot` _combatdebugwidget))) (`KismetMathLibrary.SelectInt` 2 1 (`/Game/BluePrint/Core/Combat/BP_CombatSystem.IsAbleToUseTowerUpgradeInCurrentCombat` _combatsystem))) _playeraction))
        (`/Game/BluePrint/Core/Player/BP_PlayerAction.SetCurrentSelectedSlotOnWidget` _playeraction _output_get)))))

(event `EnhancedInput|/Game/BluePrint/Core/Player/Input/IA_UpgradeTower`
  (params (ActionValue :type Boolean) (ElapsedSeconds :type "Float (double-precision)") (TriggeredSeconds :type "Float (double-precision)") (InputAction :type "InputAction Object Reference" :default "/Game/BluePrint/Core/Player/Input/IA_UpgradeTower.IA_UpgradeTower"))
  (bind _playeraction (`self.PlayerAction`))
  (bind _combatsystem (`/Game/BluePrint/Core/Player/BP_PlayerAction.CombatSystem` _playeraction))
  (bind _combatdebugwidget (`/Game/BluePrint/Core/Combat/BP_CombatSystem.CombatDebugWidget` _combatsystem))
  (:`Triggered`
    (`/Engine/EditorBlueprintResources/StandardMacros.IsValid` _combatdebugwidget
      (:`Is Valid`
        (if (`/Game/BluePrint/Core/Combat/BP_CombatSystem.IsAbleToUseTowerUpgradeInCurrentCombat` _combatsystem)
          (bind _output_get (set `/Game/BluePrint/Core/Player/BP_PlayerAction.CurrentSlotIndex` (- (`PanelWidget.GetChildrenCount` (`/Game/BluePrint/Core/Combat/DebugWidget/WBP_VerticalSlot.vBox_SlotGroup` (`/Game/BluePrint/Core/Combat/DebugWidget/WBP_DebugCombatScreen.WBP_VerticalSlot` _combatdebugwidget))) 1) _playeraction))
          (`/Game/BluePrint/Core/Player/BP_PlayerAction.SetCurrentSelectedSlotOnWidget` _playeraction _output_get))))))

(event `EnhancedInput|/Game/BluePrint/Core/Player/Input/IA_QuickChooseWeapon`
  (params (ActionValue :type Boolean) (ElapsedSeconds :type "Float (double-precision)") (TriggeredSeconds :type "Float (double-precision)") (InputAction :type "InputAction Object Reference" :default "/Game/BluePrint/Core/Player/Input/IA_QuickChooseWeapon.IA_QuickChooseWeapon"))
  (bind _playeraction (`self.PlayerAction`))
  (:`Triggered`
    (`/Engine/EditorBlueprintResources/StandardMacros.IsValid` (`/Game/BluePrint/Core/Combat/BP_CombatSystem.CombatDebugWidget` (`/Game/BluePrint/Core/Player/BP_PlayerAction.CombatSystem` _playeraction))
      (:`Is Valid`
        (bind _output_get (set `/Game/BluePrint/Core/Player/BP_PlayerAction.CurrentSlotIndex` 0 _playeraction))
        (`/Game/BluePrint/Core/Player/BP_PlayerAction.SetCurrentSelectedSlotOnWidget` _playeraction _output_get)))))

(event `EnhancedInput|/Game/BluePrint/Core/Player/Input/IA_SkipBreakTime`
  (params (ActionValue :type Boolean) (ElapsedSeconds :type "Float (double-precision)") (TriggeredSeconds :type "Float (double-precision)") (InputAction :type "InputAction Object Reference" :default "/Game/BluePrint/Core/Player/Input/IA_SkipBreakTime.IA_SkipBreakTime"))
  (:`Started`
    (`/Engine/EditorBlueprintResources/StandardMacros.DoOnce` false :!label _label
      (:`Completed`
        (`/Game/BluePrint/Core/Combat/BP_CombatSystem.SkipBreakTime` (`/Game/BluePrint/Core/Player/BP_PlayerAction.CombatSystem` (`self.PlayerAction`)))
        (`KismetSystemLibrary.PrintString` "SkipBreak Time"))))
  (:`Completed`
    (goto _label :!via `Reset`)))

(event `EnhancedInput|/Game/BluePrint/Core/Player/Input/IA_MouseLeftClick`
  (params (ActionValue :type Boolean) (ElapsedSeconds :type "Float (double-precision)") (TriggeredSeconds :type "Float (double-precision)") (InputAction :type "InputAction Object Reference" :default "/Game/BluePrint/Core/Player/Input/IA_MouseLeftClick.IA_MouseLeftClick"))
  (bind _controllercurrentstate (`/Game/BluePrint/Core/Player/BP_PlayerAction.ControllerCurrentState` (`self.PlayerAction`)))
  (:`Triggered`
    (if (and ActionValue (`|EnumInequality` _controllercurrentstate "NewEnumerator0"))
      (if (`|EnumInequality` _controllercurrentstate "NewEnumerator1")
        (`/Engine/EditorBlueprintResources/StandardMacros.DoOnce` false :!label _label_2
          (:`Completed`
            (`/Game/BluePrint/Core/Player/BP_PlayerAction.ExecuteLeftClick` (`self.PlayerAction`))
            (`KismetSystemLibrary.PrintString` "Player Unit Left Click")))
        (else
          (`/Game/BluePrint/Core/Player/BP_PlayerAction.ExecuteLeftClick` (`self.PlayerAction`))))))
  (:`Completed`
    (goto _label_2 :!via `Reset`)))

(event `EnhancedInput|/Game/BluePrint/Core/Player/Input/IA_MouseRightClick`
  (params (ActionValue :type Boolean) (ElapsedSeconds :type "Float (double-precision)") (TriggeredSeconds :type "Float (double-precision)") (InputAction :type "InputAction Object Reference" :default "/Game/BluePrint/Core/Player/Input/IA_MouseRightClick.IA_MouseRightClick"))
  (:`Triggered`
    (if (and ActionValue (`|EnumInequality` (`/Game/BluePrint/Core/Player/BP_PlayerAction.ControllerCurrentState` (`self.PlayerAction`)) "NewEnumerator0"))
      (`/Engine/EditorBlueprintResources/StandardMacros.DoOnce` false :!label _label_3
        (:`Completed`
          (`/Game/BluePrint/Core/Player/BP_PlayerAction.ExecuteRightClick` (`self.PlayerAction`))
          (`KismetSystemLibrary.PrintString` "Player Unit Right Click")))))
  (:`Completed`
    (goto _label_3 :!via `Reset`)))

(event `self.CapsuleComponent.OnComponentBeginOverlap`
  (params (OverlappedComponent :type "PrimitiveComponent Object Reference") (OtherActor :type "Actor Object Reference") (OtherComp :type "PrimitiveComponent Object Reference") (OtherBodyIndex :type Integer) (bFromSweep :type Boolean) (SweepResult :type "HitResult Structure (by ref)"))
  (cast `/Game/BluePrint/Core/Terrain/BP_DeathArea` OtherActor)
  (`self.K2_SetActorLocation` (`self.StartLocation`)))

(fn `GetCursorLocationOnTerrainFromCamera`
  (returns (Location :type "Vector Structure"))
  (bind _camera (`self.Camera`))
  (bind _returnvalue (`SceneComponent.K2_GetComponentLocation` _camera))
  (bind (_outhit _returnvalue_2) (`KismetSystemLibrary.LineTraceSingle` _returnvalue (+ _returnvalue (* (`SceneComponent.GetForwardVector` _camera) 9999999.0)) "TraceTypeQuery4"))
  (if _returnvalue_2
    (return (`.Location` (`GameplayStatics.BreakHitResult` _outhit)))
    (else
      (return (-999.0 -999.0 -999.0)))))

(fn `UserConstructionScript`
  (`parent.UserConstructionScript`))