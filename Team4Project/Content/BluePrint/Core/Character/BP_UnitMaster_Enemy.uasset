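; Base enemy unit that walks a waypoint path, with health and move speed driven by per-type data.
; Construction loads EnemyType defaults into the Data struct and resets current HP and speed.
; AI MoveTo chains through waypoints, restarting on path changes when each move ends, then stops or optionally loops.
; Modifiers update HP with floating numbers, broadcasting removal at zero, and walk speed by flat or percent amounts, using -999 as unset.
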(event `self.ReceiveBeginPlay`
  (`parent.ReceiveBeginPlay`)
  (`self.FollowTheWayPoint`))

(event `FollowTheWayPoint`
  (if (> (`KismetArrayLibrary.Array_Length` (`self.WayPointsPath`)) 0)
    (if (`self.IsWayPointPathChanged`)
      (set `self.CurrentTargetWayPointIndex` 0)
      (set `self.IsWayPointPathChanged` false))
    (`|AIMoveTo` self (100.0 0.0 0.0) (`|GetArrayItem` (`self.WayPointsPath`) (`self.CurrentTargetWayPointIndex`)) 50.0
      (:`OnSuccess`
        (if (`self.IsWayPointPathChanged`)
          (`self.FollowTheWayPoint`)
          (elif (not (>= (`self.CurrentTargetWayPointIndex`) (- (`KismetArrayLibrary.Array_Length` (`self.WayPointsPath`)) 1)))
            (set `self.CurrentTargetWayPointIndex` (+ (`self.CurrentTargetWayPointIndex`) 1))
            (`self.FollowTheWayPoint`)
            (elif (`self.IsLoopingPathTest`)
              (set `self.CurrentTargetWayPointIndex` (mod (+ (`self.CurrentTargetWayPointIndex`) 1) (`KismetArrayLibrary.Array_Length` (`self.WayPointsPath`))))
              (`self.FollowTheWayPoint`)
              (else
                (`MovementComponent.StopMovementImmediately` (`self.CharacterMovement`)))))))
      (:`OnFail`
        (`KismetSystemLibrary.PrintString` "FailToMove" false)
        (if (`self.IsWayPointPathChanged`)
          (`self.FollowTheWayPoint`))))))

(fn `ModifierCurrentHp`
  (params (Damage :type "Float (double-precision)"))
  (bind (_maxhp _currenthp) (break `/Game/BluePrint/Core/Character/Utilities_Enemy/S_EnemyNumericalStats` (`.NumerialStats_8_CC353BB04F85AD5E97CF9EA9BE9D5DE1` (break `/Game/BluePrint/Core/Character/Utilities_Enemy/S_EnemyData` (`self.Data`)))))
  (if (!= Damage 0.0)
    (`self.SetCurrentHp` (`KismetMathLibrary.FClamp` (+ _currenthp (`local.Damage`)) 0.0 _maxhp))
    (`self.SpawnEnemyAnimation` (`KismetMathLibrary.FTrunc` Damage))
    (if (<= (`.CurrentHp_7_C55A1A5E40E19DDE92A496A58C98A535` (break `/Game/BluePrint/Core/Character/Utilities_Enemy/S_EnemyNumericalStats` (`.NumerialStats_8_CC353BB04F85AD5E97CF9EA9BE9D5DE1` (break `/Game/BluePrint/Core/Character/Utilities_Enemy/S_EnemyData` (`self.Data`))))) 0.0)
      (`KismetSystemLibrary.PrintString` "CallRemoveEnemyFromCombat" false true (struct :`R` 0.572545 :`B` 1.0 :`A` 1.0) 5.0)
      (`self.OnEnemyNeedToRemoveFromCombat` self))))

(fn `ModifierCurrentMoveSpeed`
  (params (SpecificSpeedModifier :type "Float (double-precision)" :default -999.0) (PercentSpeedModifier :type "Float (double-precision)" :default -999.0))
  (if (!= SpecificSpeedModifier -999.0)
    (`self.SetCurrentMoveSpeed` (+ (`.CurrentMoveSpeed_17_B39788B64A56734BA2E01C957DD55429` (break `/Game/BluePrint/Core/Character/Utilities_Enemy/S_EnemyNumericalStats` (`.NumerialStats_8_CC353BB04F85AD5E97CF9EA9BE9D5DE1` (break `/Game/BluePrint/Core/Character/Utilities_Enemy/S_EnemyData` (`self.Data`))))) (`local.SpecificSpeedModifier`)))
    (elif (!= PercentSpeedModifier -999.0)
      (`self.SetCurrentMoveSpeed` (* (`.CurrentMoveSpeed_17_B39788B64A56734BA2E01C957DD55429` (break `/Game/BluePrint/Core/Character/Utilities_Enemy/S_EnemyNumericalStats` (`.NumerialStats_8_CC353BB04F85AD5E97CF9EA9BE9D5DE1` (break `/Game/BluePrint/Core/Character/Utilities_Enemy/S_EnemyData` (`self.Data`))))) (/ (+ 100.0 (`local.PercentSpeedModifier`)) 100.0))))))

(fn `ResetCurrentHp`
  (`self.SetCurrentHp` (`.MaxHp_6_BF564B66454D3F25F0084BBDB4A648E4` (break `/Game/BluePrint/Core/Character/Utilities_Enemy/S_EnemyNumericalStats` (`.NumerialStats_8_CC353BB04F85AD5E97CF9EA9BE9D5DE1` (break `/Game/BluePrint/Core/Character/Utilities_Enemy/S_EnemyData` (`self.Data`)))))))

(fn `ResetCurrentMoveSpeed`
  (`self.SetCurrentMoveSpeed` (`.DefaultMoveSpeed_14_6CEC3D284879072D0C3A398D9D416649` (break `/Game/BluePrint/Core/Character/Utilities_Enemy/S_EnemyNumericalStats` (`.NumerialStats_8_CC353BB04F85AD5E97CF9EA9BE9D5DE1` (break `/Game/BluePrint/Core/Character/Utilities_Enemy/S_EnemyData` (`self.Data`)))))))

(fn `SetCurrentHp`
  (params (NewCurrentHp :type "Float (double-precision)"))
  (bind _structout (setmembers `/Game/BluePrint/Core/Character/Utilities_Enemy/S_EnemyNumericalStats` :`StructRef` (`.NumerialStats_8_CC353BB04F85AD5E97CF9EA9BE9D5DE1` (break `/Game/BluePrint/Core/Character/Utilities_Enemy/S_EnemyData` (`self.Data`))) :`CurrentHp` NewCurrentHp))
  (bind _structout_2 (setmembers `/Game/BluePrint/Core/Character/Utilities_Enemy/S_EnemyData` :`StructRef` (`self.Data`) :`NumerialStats` _structout))
  (set `self.Data` _structout_2))

(fn `SetCurrentMoveSpeed`
  (params (NewCurrentSpeed :type "Float (double-precision)"))
  (bind _structout (setmembers `/Game/BluePrint/Core/Character/Utilities_Enemy/S_EnemyNumericalStats` :`StructRef` (`.NumerialStats_8_CC353BB04F85AD5E97CF9EA9BE9D5DE1` (break `/Game/BluePrint/Core/Character/Utilities_Enemy/S_EnemyData` (`self.Data`))) :`CurrentMoveSpeed` NewCurrentSpeed))
  (bind _structout_2 (setmembers `/Game/BluePrint/Core/Character/Utilities_Enemy/S_EnemyData` :`StructRef` (`self.Data`) :`NumerialStats` _structout))
  (set `self.Data` _structout_2)
  (bind _output_get (set `CharacterMovementComponent.MaxWalkSpeed` (`.CurrentMoveSpeed_17_B39788B64A56734BA2E01C957DD55429` (break `/Game/BluePrint/Core/Character/Utilities_Enemy/S_EnemyNumericalStats` (`.NumerialStats_8_CC353BB04F85AD5E97CF9EA9BE9D5DE1` (break `/Game/BluePrint/Core/Character/Utilities_Enemy/S_EnemyData` (`self.Data`))))) (`self.CharacterMovement`))))

(fn `SetEnemyData`
  (params (EnemyData :type "/Game/BluePrint/Core/Character/Utilities_Enemy/S_EnemyData Structure"))
  (set `self.Data` EnemyData)
  (`self.ResetCurrentHp`)
  (`self.ResetCurrentMoveSpeed`))

(fn `SpawnEnemyAnimation`
  (params (Number :type Integer))
  (if (!= Number 0)
    (`|SpawnActorFromClass` "/Game/BluePrint/Core/Character/Widget/BP_AnimNumber.BP_AnimNumber_C" (`KismetMathLibrary.MakeTransform` (+ (`self.K2_GetActorLocation`) (0.0 0.0 30.0))) "AlwaysSpawn" "MultiplyWithRoot" null Number null)))

(fn `UserConstructionScript`
  (`parent.UserConstructionScript`)
  (`self.SetEnemyData` (`/Game/BluePrint/Core/Character/Utilities_Enemy/BFL_Enemy.GetEnemyDefaultDataBaseOnEnemyType` (`self.EnemyType`))))