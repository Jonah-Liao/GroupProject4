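; BP_TerrainGridVisual is the visual layer of the terrain grid, showing tiles that can take towers.
; On initialization it passes the terrain's flat shape mesh and material to a child BP_TerrainMeshInst actor and centers itself at the world origin.
; Tile updates remove that index's instance, re-adding it with side transforms and states only if tower-buildable.
; Destroying the visual clears all instances; actor tick is disabled.
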(event `self.ReceiveBeginPlay`
  (`self.SetActorTickEnabled` false))

(fn `DestroyTerrainVisual`
  (bind _terrainmeshinst (`self.TerrainMeshInst`))
  (`/Engine/EditorBlueprintResources/StandardMacros.IsValid` _terrainmeshinst
    (:`Is Valid`
      (`/Game/BluePrint/Core/Terrain/BP_TerrainMeshInst.ClearInstances` _terrainmeshinst))))

(fn `InitializeTerrainVisual`
  (params (Terrain :type "/Game/BluePrint/Core/Terrain/BP_Terrain Object Reference"))
  (bind (_gridsize _mesh _meshmaterial _flatmesh _flatmaterial) (break `/Game/BluePrint/Core/Terrain/GridShape/S_GridShapeData` (`/Game/BluePrint/Core/Terrain/BP_Terrain.GetCurrentShapeData` (`self.Terrain`))))
  (set `self.Terrain` Terrain)
  (set `self.TerrainMeshInst` (cast `/Game/BluePrint/Core/Terrain/BP_TerrainMeshInst` (`ChildActorComponent.ChildActor` (`self.ChildActor_TerrainMeshInst`)) :!pure true))
  (`/Game/BluePrint/Core/Terrain/BP_TerrainMeshInst.InitializeTerrainMeshInst` (`self.TerrainMeshInst`) _flatmesh _flatmaterial (struct :`R` 0.110105 :`B` 0.398958 :`A` 1.0) "QueryOnly" null null (struct :`R` 1.0 :`G` 0.833333 :`A` 1.0) "QueryOnly" (0.0 0.0 0.0))
  (`self.K2_SetActorLocation` (0.0 0.0 0.0)) ; CenterTerrainInWorld
)

(fn `UpdateTileVisual`
  (params (TileData :type "/Game/BluePrint/Core/Terrain/Utilities/S_TileData Structure"))
  (bind (_terrainindex _tiletype _transformofallside _statesofallsidetiles) (break `/Game/BluePrint/Core/Terrain/Utilities/S_TileData` (`local.TileData`)))
  (`/Game/BluePrint/Core/Terrain/BP_TerrainMeshInst.RemoveInstance` (`self.TerrainMeshInst`) _terrainindex)
  (if (`/Game/BluePrint/Core/Terrain/Utilities/BFL_TileData.IsTileTowerBuildable` _tiletype)
    (`/Game/BluePrint/Core/Terrain/BP_TerrainMeshInst.AddInstance` (`self.TerrainMeshInst`) _terrainindex _transformofallside _statesofallsidetiles)))

(fn `UserConstructionScript`)