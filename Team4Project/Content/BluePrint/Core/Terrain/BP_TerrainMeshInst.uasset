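; BP_TerrainMeshInst renders grid terrain as six instanced static meshes, one per side (top, bottom, front, back, left, right).
; InitializeTerrainMeshInst applies the flat mesh, material, color and collision to all six, leaving cube inputs unused.
; Per-side index arrays parallel the instances, letting AddInstance replace and RemoveInstance delete by terrain index.
; Per-instance custom data carries highlight color and fill from tile states, with Selected overriding Hovered.
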(fn `AddInstance`
  (params (TerrainIndex :type "IntVector Structure") (TerrainTransform :type "/Game/BluePrint/Core/Terrain/Utilities/S_SidesOfGridTransform Structure") (AllSideTileStates :type "/Game/BluePrint/Core/Terrain/Utilities/S_AllSideTilesStates Structure"))
  (locals (I :type Integer :default 0) (TempIndexArray :type "Array of IntVector Structure") (SideIndex :type Integer))
  (bind (_top _bottom _front _back _left _right) (break `/Game/BluePrint/Core/Terrain/Utilities/S_SidesOfGridTransform` TerrainTransform))
  (bind (_top_tilestates _bottom_tilestates _front_tilestates _back_tilestates _left_tilestates _right_tilestates) (break `/Game/BluePrint/Core/Terrain/Utilities/S_AllSideTilesStates` AllSideTileStates))
  (bind _i (`local.I`))
  (bind _s_indexarrayofgridside (make `/Game/BluePrint/Core/Terrain/Utilities/S_IndexArrayOfGridSide` (`local.TempIndexArray`)))
  (`|ExecutionSequence`
    (:`then_0`
      (`self.RemoveInstance` TerrainIndex))
    (:`then_1`
      (for (_array_element _array_index) (`|MakeArray` (`self.InstancedStaticMesh_Top`) (`self.InstancedStaticMesh_Bottom`) (`self.InstancedStaticMesh_Front`) (`self.InstancedStaticMesh_Back`) (`self.InstancedStaticMesh_Left`) (`self.InstancedStaticMesh_Right`))
        (set `local.SideIndex` _array_index)
        (bind _returnvalue (`InstancedStaticMeshComponent.AddInstance` _array_element (`|GetArrayItem` (`|MakeArray` _top _bottom _front _back _left _right) (`local.SideIndex`)) false))
        (set `local.I` _returnvalue)
        (bind _output_get (set `local.TempIndexArray` (`.IntVectorArray_15_1E67F0264EEAAD7D408B23A672134902` (break `/Game/BluePrint/Core/Terrain/Utilities/S_IndexArrayOfGridSide` (`|GetArrayItem` (`|MakeArray` (`self.TerrainIndex_Top`) (`self.TerrainIndex_Bottom`) (`self.TerrainIndex_Front`) (`self.TerrainIndex_Back`) (`self.TerrainIndex_Left`) (`self.TerrainIndex_Right`)) (`local.SideIndex`))))))
        (`KismetArrayLibrary.Array_Add` _output_get (`local.TerrainIndex`))
        (`|ExecutionSequence`
          (:`then_0`
            (switch `int` (`local.SideIndex`)
              (:`0`
                (set `self.TerrainIndex_Top` _s_indexarrayofgridside))
              (:`1`
                (set `self.TerrainIndex_Bottom` _s_indexarrayofgridside))
              (:`2`
                (set `self.TerrainIndex_Front` _s_indexarrayofgridside))
              (:`3`
                (set `self.TerrainIndex_Back` _s_indexarrayofgridside))
              (:`4`
                (set `self.TerrainIndex_Left` _s_indexarrayofgridside))
              (:`5`
                (set `self.TerrainIndex_Right` _s_indexarrayofgridside))))
          (:`then_1`
            (bind (_color _isfilled) (`self.GetColorFromTileStates` (`.CurrentTileStates_4_AF7836E0465DE217633BFCB58FD3FE78` (break `/Game/BluePrint/Core/Terrain/Utilities/S_TileStateArray` (`|GetArrayItem` (`|MakeArray` _top_tilestates _bottom_tilestates _front_tilestates _back_tilestates _left_tilestates _right_tilestates) (`local.SideIndex`))))))
            (bind (_r _g _b) (break `LinearColor` _color))
            (`InstancedStaticMeshComponent.SetCustomDataValue` _array_element _i 0 _r false)
            (`InstancedStaticMeshComponent.SetCustomDataValue` _array_element _i 1 _g false)
            (`InstancedStaticMeshComponent.SetCustomDataValue` _array_element _i 2 _b false)
            (`InstancedStaticMeshComponent.SetCustomDataValue` _array_element _i 3 _isfilled false)))))))

(fn `ClearInstances`
  (`InstancedStaticMeshComponent.ClearInstances` (`self.InstancedStaticMesh_Top`))
  (`InstancedStaticMeshComponent.ClearInstances` (`self.InstancedStaticMesh_Front`))
  (`InstancedStaticMeshComponent.ClearInstances` (`self.InstancedStaticMesh_Back`))
  (`InstancedStaticMeshComponent.ClearInstances` (`self.InstancedStaticMesh_Bottom`))
  (`InstancedStaticMeshComponent.ClearInstances` (`self.InstancedStaticMesh_Left`))
  (`InstancedStaticMeshComponent.ClearInstances` (`self.InstancedStaticMesh_Right`))
  (set `self.TerrainIndex_Top` (struct))
  (set `self.TerrainIndex_Bottom` (struct))
  (set `self.TerrainIndex_Front` (struct))
  (set `self.TerrainIndex_Back` (struct))
  (set `self.TerrainIndex_Left` (struct))
  (set `self.TerrainIndex_Right` (struct)))

(fn `GetColorFromTileStates`
  (params (States :type "Array of /Game/BluePrint/Core/Terrain/Utilities/Enum_TileState Enum"))
  (returns (Color :type "LinearColor Structure") (IsFilled :type "Float (double-precision)"))
  (if (== (`KismetArrayLibrary.Array_Length` States) 0)
    (return (struct :`A` 1.0) 0.0)
    (else
      (for _array_element (`|MakeArray` "NewEnumerator2" "NewEnumerator1" :!type "/Game/BluePrint/Core/Terrain/Utilities/Enum_TileState Enum")
        (if (`KismetArrayLibrary.Array_Contains` (`local.States`) _array_element)
          (return (select `/Game/BluePrint/Core/Terrain/Utilities/Enum_TileState` _array_element :`NewEnumerator0` (struct :`A` 1.0) :`NewEnumerator1` (struct :`R` 1.0 :`G` 0.49423 :`A` 1.0) :`NewEnumerator2` (struct :`G` 1.0 :`B` 0.844667 :`A` 1.0) :!type "LinearColor Structure") 1.0)))
      (return (struct) 0.0))))

(fn `InitializeTerrainMeshInst`
  (params (FlatMesh :type "StaticMesh Object Reference") (FlatMaterial :type "MaterialInterface Object Reference") (FlatColor :type "LinearColor Structure") (FlatCollision :type "ECollisionEnabled Enum" :default "NoCollision") (CubeMesh :type "StaticMesh Object Reference") (CubeMaterial :type "MaterialInterface Object Reference") (CubeColor :type "LinearColor Structure" :default (struct :`R` 1.0 :`G` 0.833333 :`A` 1.0)) (CubeCollision :type "ECollisionEnabled Enum" :default "NoCollision") (GridSize :type "Vector Structure"))
  (for _array_element (`|MakeArray` (`self.InstancedStaticMesh_Top`) (`self.InstancedStaticMesh_Bottom`) (`self.InstancedStaticMesh_Front`) (`self.InstancedStaticMesh_Back`) (`self.InstancedStaticMesh_Left`) (`self.InstancedStaticMesh_Right`))
    (`StaticMeshComponent.SetStaticMesh` _array_element FlatMesh)
    (`PrimitiveComponent.SetMaterial` _array_element 0 FlatMaterial)
    (`MeshComponent.SetVectorParameterValueOnMaterials` _array_element "Color" (`KismetMathLibrary.Conv_LinearColorToVector` FlatColor))
    (`PrimitiveComponent.SetCollisionEnabled` _array_element FlatCollision)))

(fn `RemoveInstance`
  (params (TerrainIndex :type "IntVector Structure"))
  (locals (TempIndexArray :type "Array of IntVector Structure") (SideIndex :type Integer))
  (bind _terrainindex (`local.TerrainIndex`))
  (bind _s_indexarrayofgridside (make `/Game/BluePrint/Core/Terrain/Utilities/S_IndexArrayOfGridSide` (`local.TempIndexArray`)))
  (for (_array_element _array_index) (`|MakeArray` (`self.TerrainIndex_Top`) (`self.TerrainIndex_Bottom`) (`self.TerrainIndex_Front`) (`self.TerrainIndex_Back`) (`self.TerrainIndex_Left`) (`self.TerrainIndex_Right`))
    (set `local.SideIndex` _array_index)
    (bind _output_get (set `local.TempIndexArray` (`.IntVectorArray_15_1E67F0264EEAAD7D408B23A672134902` (break `/Game/BluePrint/Core/Terrain/Utilities/S_IndexArrayOfGridSide` _array_element))))
    (if (`KismetArrayLibrary.Array_Contains` _output_get _terrainindex)
      (`InstancedStaticMeshComponent.RemoveInstance` (`|GetArrayItem` (`|MakeArray` (`self.InstancedStaticMesh_Top`) (`self.InstancedStaticMesh_Bottom`) (`self.InstancedStaticMesh_Front`) (`self.InstancedStaticMesh_Back`) (`self.InstancedStaticMesh_Left`) (`self.InstancedStaticMesh_Right`)) (`local.SideIndex`)) (`KismetArrayLibrary.Array_Find` _output_get _terrainindex))
      (bind _returnvalue (`KismetArrayLibrary.Array_RemoveItem` (`local.TempIndexArray`) (`local.TerrainIndex`)))
      (if _returnvalue
        (switch `int` (`local.SideIndex`)
          (:`0`
            (set `self.TerrainIndex_Top` _s_indexarrayofgridside))
          (:`1`
            (set `self.TerrainIndex_Bottom` _s_indexarrayofgridside))
          (:`2`
            (set `self.TerrainIndex_Front` _s_indexarrayofgridside))
          (:`3`
            (set `self.TerrainIndex_Back` _s_indexarrayofgridside))
          (:`4`
            (set `self.TerrainIndex_Left` _s_indexarrayofgridside))
          (:`5`
            (set `self.TerrainIndex_Right` _s_indexarrayofgridside)))))))

(fn `UserConstructionScript`)