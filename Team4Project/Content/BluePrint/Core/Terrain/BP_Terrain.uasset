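; BP_Terrain builds a snapped 3D grid of tower-buildable terrain tiles around a center location.
; SpawnTerrain clears old instances, then forms each tile from six Instanced Static Mesh faces, using mesh and material from the grid shape's data.
; With environment use on, downward sphere traces snap tile height to the ground and skip misses or obstacles marked by BP_TerrainModifier.
; The construction script's SpawnTerrain call is disconnected, so nothing here triggers generation.
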(event `self.ReceiveBeginPlay`)

(fn `CalculateCenterAndBottomLeft`
  (returns (SnapGridTerrainCenter :type "Vector Structure") (SnapGridBottomLeftCenter :type "Vector Structure"))
  (locals (C :type "Vector Structure" :default (0.0 0.0 0.0)))
  (bind (_x _y) (break `IntVector` (`self.TerrainTileCount`)))
  (bind (_x_2 _y_2) (break `IntVector` (`self.TerrainTileCount`)))
  (set `local.C` (`/Game/BluePrint/Core/Utilities/BFL_Utilities.SnapVectorToCriterion` (`self.TerrainCenterLocation`) (`self.TerrainGridSize`)))
  (return (`local.C`) (- (`local.C`) (`KismetMathLibrary.MakeVector` (* (/ (- _x (select `bool` (`/Game/BluePrint/Core/Utilities/BFL_Utilities.IsIntEven` _x_2) :`false` 1)) 2) (.x (`self.TerrainGridSize`))) (* (/ (- _y (select `bool` (`/Game/BluePrint/Core/Utilities/BFL_Utilities.IsIntEven` _y_2) :`false` 1)) 2) (.y (`self.TerrainGridSize`)))))))

(fn `DestroyTerrain`
  (`InstancedStaticMeshComponent.ClearInstances` (`self.InstancedStaticMesh_Right`))
  (`InstancedStaticMeshComponent.ClearInstances` (`self.InstancedStaticMesh_Top`))
  (`InstancedStaticMeshComponent.ClearInstances` (`self.InstancedStaticMesh_Bottom`))
  (`InstancedStaticMeshComponent.ClearInstances` (`self.InstancedStaticMesh_Front`))
  (`InstancedStaticMeshComponent.ClearInstances` (`self.InstancedStaticMesh_Back`))
  (`InstancedStaticMeshComponent.ClearInstances` (`self.InstancedStaticMesh_Left`)))

(fn `GetCurrentShapeData`
  (returns (ReturnValue :type "/Game/BluePrint/Core/Terrain/GridShape/S_GridShapeData Structure"))
  (return (`/Game/BluePrint/Core/Terrain/GridShape/BFL_GridShape.GetGridShapeData` (`self.TerrainGridShape`))))

(fn `GetTileLocationFromGridIndex`
  (params (GridIndex :type "IntVector Structure (by ref)"))
  (returns (TargetLocation :type "Vector Structure"))
  (bind (_x _y _z) (break `IntVector` GridIndex))
  (return (+ (`self.TerrainBottomLeftLocation`) (`KismetMathLibrary.MakeVector` (* _x (.x (`self.TerrainGridSize`))) (* _y (.y (`self.TerrainGridSize`))) (* _z (.z (`self.TerrainGridSize`)))))))

(fn `GetTileRotationFromGridIndex`
  (params (GridIndex :type "IntVector Structure"))
  (returns (TargetRotation :type "Rotator Structure"))
  (switch `/Game/BluePrint/Core/Terrain/GridShape/Enum_GridShape` (`self.TerrainGridShape`)
    (:`NewEnumerator0`
      _)
    (:`NewEnumerator1`
      _))
  (return))

(fn `IsTileTypeTowerBuildable`
  (params (TileType :type "/Game/BluePrint/Core/Terrain/Utilities/Enum_TileType Enum" :default "NewEnumerator0"))
  (returns (IsTowerBuildable :type Boolean))
  (return (select `/Game/BluePrint/Core/Terrain/Utilities/Enum_TileType` TileType :`NewEnumerator1` true)))

(fn `SetGridOffsetFromGround`
  (params (TransformOffset :type "Float (double-precision)")))

(fn `SetTileOffsetAndTransformDeltaBaseOnTilePivot`
  (params (Offset :type "Float (double-precision)"))
  (returns (Top :type "Transform Structure") (Bottom :type "Transform Structure") (Front :type "Transform Structure") (Back :type "Transform Structure") (Left :type "Transform Structure") (Right :type "Transform Structure"))
  (locals (TileTopBaseOnTilePivot :type "Transform Structure"))
  (return (`KismetMathLibrary.MakeTransform` (`KismetMathLibrary.MakeVector` 0.0 0.0 (`local.Offset`))) (`KismetMathLibrary.MakeTransform` (`KismetMathLibrary.MakeVector` 0.0 0.0 (- 0.0 (.z (`self.TerrainGridSize`)) (`local.Offset`)))) (`KismetMathLibrary.MakeTransform` (`KismetMathLibrary.MakeVector` (+ (/ (.x (`self.TerrainGridSize`)) 2.0) (`local.Offset`)) 0.0 (- 0.0 (/ (.z (`self.TerrainGridSize`)) 2.0))) (struct :`Pitch` -90.0)) (`KismetMathLibrary.MakeTransform` (`KismetMathLibrary.MakeVector` (- 0.0 (/ (.x (`self.TerrainGridSize`)) 2.0) (`local.Offset`)) 0.0 (- 0.0 (/ (.z (`self.TerrainGridSize`)) 2.0))) (struct :`Pitch` -90.0)) (`KismetMathLibrary.MakeTransform` (`KismetMathLibrary.MakeVector` 0.0 (- 0.0 (/ (.y (`self.TerrainGridSize`)) 2.0) (`local.Offset`)) (- 0.0 (/ (.z (`self.TerrainGridSize`)) 2.0))) (struct :`Roll` 90.0)) (`KismetMathLibrary.MakeTransform` (`KismetMathLibrary.MakeVector` 0.0 (+ (/ (.y (`self.TerrainGridSize`)) 2.0) (`local.Offset`)) (- 0.0 (/ (.z (`self.TerrainGridSize`)) 2.0))) (struct :`Roll` 90.0))))

(fn `SpawnTerrain`
  (params (CenterLocation :type "Vector Structure") (GridSize :type "Vector Structure") (TileCount :type "IntVector Structure") (Shape :type "/Game/BluePrint/Core/Terrain/GridShape/Enum_GridShape Enum" :default "NewEnumerator0") (TileOffsetFromTerrain :type "Float (double-precision)") (UseEnvironment :type Boolean))
  (locals (X :type Integer) (Y :type Integer) (Z :type Integer) (TileIndex :type "IntVector Structure") (TileTransform :type "Transform Structure") (TileTopBaseOnTilePivot :type "Transform Structure") (TileBottomBaseOnTilePivot :type "Transform Structure") (TileFrontBaseOnTilePivot :type "Transform Structure") (TileBackBaseOnTilePivot :type "Transform Structure") (TileLeftBaseOnTilePivot :type "Transform Structure") (TileRightBaseOnTilePivot :type "Transform Structure"))
  (bind ((`FlatMesh_14_AA1283DC46A9ADB73358FEA9FCD07807` _flatmesh) (`FlatMaterial_15_3057BC754CCA52F2D6703AB0A02CA972` _flatmaterial)) (break `/Game/BluePrint/Core/Terrain/GridShape/S_GridShapeData` (`self.GetCurrentShapeData`)))
  (set `self.TerrainCenterLocation` CenterLocation)
  (set `self.TerrainGridSize` GridSize)
  (set `self.TerrainTileCount` TileCount)
  (set `self.TerrainGridShape` Shape)
  (set `self.CurrentTileOffsetFromTerrain` TileOffsetFromTerrain)
  (set `self.IsUseEnvironment` UseEnvironment)
  (`self.DestroyTerrain`)
  (for _array_element (`|MakeArray` (`self.InstancedStaticMesh_Top`) (`self.InstancedStaticMesh_Bottom`) (`self.InstancedStaticMesh_Front`) (`self.InstancedStaticMesh_Back`) (`self.InstancedStaticMesh_Left`) (`self.InstancedStaticMesh_Right`))
    (`StaticMeshComponent.SetStaticMesh` _array_element _flatmesh)
    (`PrimitiveComponent.SetMaterial` _array_element 0 _flatmaterial)
    (bind (_snapgridterraincenter _snapgridbottomleftcenter) (`self.CalculateCenterAndBottomLeft`))
    (set `self.TerrainCenterLocation` _snapgridterraincenter)
    (set `self.TerrainBottomLeftLocation` _snapgridbottomleftcenter)
    (for _index (range (`.X` (break `IntVector` (`self.TerrainTileCount`))))
      (set `local.X` _index)
      (for _index_2 (range (`.Y` (break `IntVector` (`self.TerrainTileCount`))))
        (set `local.Y` _index_2)
        (for _index_3 (range (`.Z` (break `IntVector` (`self.TerrainTileCount`))))
          (set `local.Z` _index_3)
          (set `local.TileIndex` (make `IntVector` (`local.X`) (`local.Y`) (`local.Z`)))
          (set `local.TileTransform` (`KismetMathLibrary.MakeTransform` (`self.GetTileLocationFromGridIndex` (`local.TileIndex`)) (`self.GetTileRotationFromGridIndex` (`local.TileIndex`)) (/ (`self.TerrainGridSize`) (`.GridSize_2_B3D3CA84488230A1876B0D9B5103CEA9` (break `/Game/BluePrint/Core/Terrain/GridShape/S_GridShapeData` (`self.GetCurrentShapeData`))))))
          (if (`self.IsUseEnvironment`)
            (bind (_tiletype _hitlocation) (`self.TraceForTerrain` (.location (`local.TileTransform`))))
            (if (`self.IsTileTypeTowerBuildable` _tiletype)
              (set `local.TileTransform` (`KismetMathLibrary.MakeTransform` _hitlocation (.rotation (`local.TileTransform`)) (.scale (`local.TileTransform`))))
              (bind (_top _bottom _front _back _left _right) (`self.SetTileOffsetAndTransformDeltaBaseOnTilePivot` (`local.TileOffsetFromTerrain`) :!label _label))
              (set `local.TileTopBaseOnTilePivot` _top)
              (set `local.TileBottomBaseOnTilePivot` _bottom)
              (set `local.TileFrontBaseOnTilePivot` _front)
              (set `local.TileBackBaseOnTilePivot` _back)
              (set `local.TileLeftBaseOnTilePivot` _left)
              (set `local.TileRightBaseOnTilePivot` _right)
              (for (_array_element_2 _array_index) (`|MakeArray` (`self.InstancedStaticMesh_Top`) (`self.InstancedStaticMesh_Bottom`) (`self.InstancedStaticMesh_Front`) (`self.InstancedStaticMesh_Back`) (`self.InstancedStaticMesh_Left`) (`self.InstancedStaticMesh_Right`))
                (`InstancedStaticMeshComponent.AddInstance` _array_element_2 (`KismetMathLibrary.MakeTransform` (+ (.location (`local.TileTransform`)) (.location (`|GetArrayItem` (`|MakeArray` (`local.TileTopBaseOnTilePivot`) (`local.TileBottomBaseOnTilePivot`) (`local.TileFrontBaseOnTilePivot`) (`local.TileBackBaseOnTilePivot`) (`local.TileLeftBaseOnTilePivot`) (`local.TileRightBaseOnTilePivot`)) _array_index))) (`KismetMathLibrary.ComposeRotators` (.rotation (`local.TileTransform`)) (.rotation (`|GetArrayItem` (`|MakeArray` (`local.TileTopBaseOnTilePivot`) (`local.TileBottomBaseOnTilePivot`) (`local.TileFrontBaseOnTilePivot`) (`local.TileBackBaseOnTilePivot`) (`local.TileLeftBaseOnTilePivot`) (`local.TileRightBaseOnTilePivot`)) _array_index))) (.scale (`local.TileTransform`))) true)))
            (else
              (goto _label))))))))

(fn `TraceForTerrain`
  (params (Location :type "Vector Structure"))
  (returns (TileType :type "/Game/BluePrint/Core/Terrain/Utilities/Enum_TileType Enum") (HitLocation :type "Vector Structure"))
  (locals (Radius :type "Float (double-precision)") (RetTileType :type "/Game/BluePrint/Core/Terrain/Utilities/Enum_TileType Enum" :default "NewEnumerator0") (Z :type "Float (double-precision)" :default 0.0))
  (bind _location (`local.Location`))
  (set `local.Radius` (/ (.z (`self.TerrainGridSize`)) 5.0))
  (bind (_outhit _returnvalue) (`KismetSystemLibrary.SphereTraceSingle` :`Start` (- _location (`KismetMathLibrary.MakeVector` 0.0 0.0 (+ (`local.Radius`) 1.0))) :`End` (- _location (`KismetMathLibrary.MakeVector` 0.0 0.0 (.z (/ (`self.TerrainGridSize`) 2.0)))) :`Radius` (`local.Radius`) :`TraceChannel` "TraceTypeQuery3" :`DrawTime` 10.0))
  (if _returnvalue
    (set `local.RetTileType` "NewEnumerator1")
    (`|ExecutionSequence`
      (:`then_0`
        (bind (_bblockinghit _binitialoverlap _time _distance _location_2 _impactpoint _normal _impactnormal _physmat _hitactor) (`GameplayStatics.BreakHitResult` _outhit))
        (bind _asbp_terrain_modifier (cast `/Game/BluePrint/Core/Terrain/BP_TerrainModifier` _hitactor))
        (set `local.RetTileType` (`/Game/BluePrint/Core/Terrain/BP_TerrainModifier.TileType` _asbp_terrain_modifier)))
      (:`then_1`
        (set `local.Z` (`KismetMathLibrary.GridSnap_Float` (.z _location_2) (.z (`self.TerrainGridSize`))))
        (return (`local.RetTileType`) (`KismetMathLibrary.MakeVector` (.x (`local.Location`)) (.y (`local.Location`)) (`local.Z`)))))
    (else
      (return "NewEnumerator0" (`local.Location`)))))

(fn `UserConstructionScript`)