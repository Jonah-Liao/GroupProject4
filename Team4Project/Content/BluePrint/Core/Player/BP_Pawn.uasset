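; Free-camera pawn with spring-arm zoom, panning, yaw and pitch, driven by Enhanced Input.
; On BeginPlay it links to BP_UnitMaster_Player and hands possession to it when no BP_DebugMenu exists.
; Otherwise, or without a player unit, it shows the cursor, adds the input mapping and starts the camera.
; Inputs only change desired values; a looping timer interpolates the actor and spring arm toward them.
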(event `self.ReceiveBeginPlay`
  (bind _returnvalue (`GameplayStatics.GetPlayerController` 0))
  (bind _returnvalue_2 (pcsubsystem `EnhancedInputLocalPlayerSubsystem` (`GameplayStatics.GetPlayerController` 0)))
  (`self.InitialCameraDesiredData`)
  ;[0 0 0 0.5] 获取地图中玩家角色蓝图并提升为变量，判断变量是否有效
  (bind _returnvalue_3 (`GameplayStatics.GetActorOfClass` "/Game/BluePrint/Core/Character/BP_UnitMaster_Player.BP_UnitMaster_Player_C"))
  (bind _output_get (set `self.Unit_Master_Player` _returnvalue_3))
  (`/Engine/EditorBlueprintResources/StandardMacros.IsValid` _output_get
    (:`Is Valid`
      (set `/Game/BluePrint/Core/Character/BP_UnitMaster_Player.Pawn` self _output_get)
      (bind _returnvalue_4 (`GameplayStatics.GetActorOfClass` "/Game/BluePrint/Core/Debug/BP_DebugMenu.BP_DebugMenu_C"))
      (bind _output_get_2 (set `self.DebugMenu` _returnvalue_4))
      (`/Engine/EditorBlueprintResources/StandardMacros.IsValid` _output_get_2
        (:`Is Valid`
          ;[0 0 0 0.5] 玩家蓝图有效则让玩家蓝图直接接受控制并隐藏鼠标
          ; 否则显示鼠标并且导入控制器键位
          (set `PlayerController.bShowMouseCursor` true (`GameplayStatics.GetPlayerController` 0) :!label _label)
          (`self.StartToUpdateCamera`)
          (`/Engine/EditorBlueprintResources/StandardMacros.IsValid` _returnvalue_2
            (:`Is Valid`
              (`EnhancedInputSubsystemInterface.AddMappingContext` _returnvalue_2 "/Game/BluePrint/Core/Player/Input/IMC_PlayerAction.IMC_PlayerAction" 0 (struct)))))
        (:`Is Not Valid`
          (`Controller.Possess` _returnvalue (`self.Unit_Master_Player`))
          (set `PlayerController.bShowMouseCursor` false _returnvalue))))
    (:`Is Not Valid`
      (goto _label))))

(event `InitialCameraDesiredData`
  ; Comment
  (set `self.Zoom_Desired` (`SpringArmComponent.TargetArmLength` (`self.SpringArm`)))
  (set `self.Location_Desired` (`self.K2_GetActorLocation`))
  (set `self.RotationLR_Desired` (`self.K2_GetActorRotation`))
  (set `self.RotationUpDown_Desired` (`SceneComponent.RelativeRotation` (`self.SpringArm`))))

(event `StartToUpdateCamera`
  ; Comment
  (bind _returnvalue (`KismetSystemLibrary.K2_SetTimerDelegate` (delegate `UpdateCamera`) (`self.DeltaTime`) true))
  (set `self.CameraUpdateTimer` _returnvalue))

(event `UpdateCamera`
  (bind _springarm (`self.SpringArm`))
  (bind _springarm_2 (`self.SpringArm`))
  ; Comment
  (set `SpringArmComponent.TargetArmLength` (`KismetMathLibrary.FInterpTo` (`SpringArmComponent.TargetArmLength` _springarm) (`self.Zoom_Desired`) (`self.DeltaTime`) (`self.Zoom_Interp`)) _springarm)
  (`self.K2_SetActorLocation` (`KismetMathLibrary.VInterpTo` (`self.K2_GetActorLocation`) (`self.Location_Desired`) (`self.DeltaTime`) (`self.Location_Interp`)))
  (`self.K2_SetActorRotation` (`KismetMathLibrary.RInterpTo` (`self.K2_GetActorRotation`) (`self.RotationLR_Desired`) (`self.DeltaTime`) (`self.Rotation_Interp`)) true)
  (`SceneComponent.K2_SetRelativeRotation` _springarm_2 (`KismetMathLibrary.RInterpTo` (`SceneComponent.RelativeRotation` _springarm_2) (`self.RotationUpDown_Desired`) (`self.DeltaTime`) (`self.Rotation_Interp`)) false false))

(event `EnhancedInput|/Game/BluePrint/Core/Player/Input/IA_AxisZoom`
  (params (ActionValue :type "Float (double-precision)") (ElapsedSeconds :type "Float (double-precision)") (TriggeredSeconds :type "Float (double-precision)") (InputAction :type "InputAction Object Reference" :default "/Game/BluePrint/Core/Player/Input/IA_AxisZoom.IA_AxisZoom"))
  ; Comment
  (:`Triggered`
    (set `self.Zoom_Desired` (`KismetMathLibrary.FClamp` (+ (* ActionValue (`self.Zoom_Speed`)) (`self.Zoom_Desired`)) (`self.Zoom_Min`) (`self.Zoom_Max`)))))

(event `EnhancedInput|/Game/BluePrint/Core/Player/Input/IA_AxisForward`
  (params (ActionValue :type "Float (double-precision)") (ElapsedSeconds :type "Float (double-precision)") (TriggeredSeconds :type "Float (double-precision)") (InputAction :type "InputAction Object Reference" :default "/Game/BluePrint/Core/Player/Input/IA_AxisForward.IA_AxisForward"))
  ; Comment
  (:`Triggered`
    (set `self.Location_Desired` (+ (`self.Location_Desired`) (* (* ActionValue (`self.Location_Speed`)) (`self.GetActorForwardVector`))))))

(event `EnhancedInput|/Game/BluePrint/Core/Player/Input/IA_AxisRight`
  (params (ActionValue :type "Float (double-precision)") (ElapsedSeconds :type "Float (double-precision)") (TriggeredSeconds :type "Float (double-precision)") (InputAction :type "InputAction Object Reference" :default "/Game/BluePrint/Core/Player/Input/IA_AxisRight.IA_AxisRight"))
  ; Comment
  (:`Triggered`
    (set `self.Location_Desired` (+ (`self.Location_Desired`) (* (* ActionValue (`self.Location_Speed`)) (`self.GetActorRightVector`))))))

(event `EnhancedInput|/Game/BluePrint/Core/Player/Input/IA_AxisRotationLeft`
  (params (ActionValue :type Boolean) (ElapsedSeconds :type "Float (double-precision)") (TriggeredSeconds :type "Float (double-precision)") (InputAction :type "InputAction Object Reference" :default "/Game/BluePrint/Core/Player/Input/IA_AxisRotationLeft.IA_AxisRotationLeft"))
  ; Comment
  (:`Started`
    (set `self.RotationLR_Desired` (`KismetMathLibrary.ComposeRotators` (`self.RotationLR_Desired`) (`KismetMathLibrary.MakeRotator` 0.0 0.0 (`self.Rotation_Speed`))))))

(event `EnhancedInput|/Game/BluePrint/Core/Player/Input/IA_AxisRotationRight`
  (params (ActionValue :type Boolean) (ElapsedSeconds :type "Float (double-precision)") (TriggeredSeconds :type "Float (double-precision)") (InputAction :type "InputAction Object Reference" :default "/Game/BluePrint/Core/Player/Input/IA_AxisRotationRight.IA_AxisRotationRight"))
  ; Comment
  (:`Started`
    (set `self.RotationLR_Desired` (`KismetMathLibrary.ComposeRotators` (`self.RotationLR_Desired`) (`KismetMathLibrary.MakeRotator` 0.0 0.0 (- 0.0 (`self.Rotation_Speed`)))))))

(event `EnhancedInput|/Game/BluePrint/Core/Player/Input/IA_AxisRotationDown`
  (params (ActionValue :type Boolean) (ElapsedSeconds :type "Float (double-precision)") (TriggeredSeconds :type "Float (double-precision)") (InputAction :type "InputAction Object Reference" :default "/Game/BluePrint/Core/Player/Input/IA_AxisRotationDown.IA_AxisRotationDown"))
  ; Comment
  (:`Triggered`
    (set `self.RotationUpDown_Desired` (`KismetMathLibrary.ComposeRotators` (`self.RotationUpDown_Desired`) (`KismetMathLibrary.MakeRotator` 0.0 (- 0.0 (`self.Rotation_UpDownSpeed`)))))))

(event `EnhancedInput|/Game/BluePrint/Core/Player/Input/IA_AxisRotationUp`
  (params (ActionValue :type Boolean) (ElapsedSeconds :type "Float (double-precision)") (TriggeredSeconds :type "Float (double-precision)") (InputAction :type "InputAction Object Reference" :default "/Game/BluePrint/Core/Player/Input/IA_AxisRotationUp.IA_AxisRotationUp"))
  ; Comment
  (:`Triggered`
    (set `self.RotationUpDown_Desired` (`KismetMathLibrary.ComposeRotators` (`self.RotationUpDown_Desired`) (`KismetMathLibrary.MakeRotator` 0.0 (`self.Rotation_UpDownSpeed`))))))

(fn `UserConstructionScript`)