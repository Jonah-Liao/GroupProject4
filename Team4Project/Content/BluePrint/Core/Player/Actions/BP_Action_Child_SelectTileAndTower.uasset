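; Player action that selects a terrain tile and, going by its name, the tower on it.
; ExecuteAction passes the tile index and side index map to PlayerActions.SetSelectedTileAndTower without forcing.
; EndPlay removes the selection state from the selected tile group on the Terrain and empties the stored selection.
; An inline version of the select and deselect logic remains in the graph but is disconnected.
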(event `self.ReceiveDestroyed`)

(event `self.ReceiveEndPlay`
  (params (EndPlayReason :type "EEndPlayReason Enum" :default "Destroyed"))
  (bind _playeractions (`self.PlayerActions`))
  (if (> (`BlueprintMapLibrary.Map_Length` (`/Game/BluePrint/Core/Player/BP_PlayerAction.SelectedTileIndexAndTileSideIndex` (`self.PlayerActions`))) 0)
    (`/Game/BluePrint/Core/Terrain/BP_Terrain.RemoveStateFromTilesGroup` (`/Game/BluePrint/Core/Player/BP_PlayerAction.Terrain` _playeractions) (`/Game/BluePrint/Core/Player/BP_PlayerAction.SelectedTileIndexAndTileSideIndex` _playeractions) "NewEnumerator2")
    (set `/Game/BluePrint/Core/Player/BP_PlayerAction.SelectedTileIndexAndTileSideIndex` (`|MakeMap`) (`self.PlayerActions`))))

(fn `ExecuteAction`
  (params (TerrainIndexAndSideTileIndex :type "Map of IntVector Structure to Integer"))
  (`/Game/BluePrint/Core/Player/BP_PlayerAction.SetSelectedTileAndTower` (`self.PlayerActions`) TerrainIndexAndSideTileIndex false))

(fn `UserConstructionScript`
  (`parent.UserConstructionScript`))