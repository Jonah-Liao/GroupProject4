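; BP_Action_WeaponShoot is a player action that fires the unit's weapon at the currently aimed enemy.
; ExecuteAction requires a valid player unit that is not reloading, then spends one round from PlayerActions, refreshes the combat debug widget and starts the reload timer on empty.
; A separate Sequence branch applies fixed HP damage directly to AimingEnemy, independent of the ammo check, and prints the target's name.
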(event `self.ReceiveDestroyed`)

(event `self.ReceiveEndPlay`
  (params (EndPlayReason :type "EEndPlayReason Enum" :default "Destroyed")))

(fn `ExecuteAction`
  (params (TerrainIndexAndSideTileIndex :type "Map of IntVector Structure to Integer"))
  (bind _playeractions (`self.PlayerActions`))
  (bind _playeractions_2 (`self.PlayerActions`))
  (bind _playeractions_3 (`self.PlayerActions`))
  (bind _playeractions_4 (`self.PlayerActions`))
  (bind _aimingenemy (`/Game/BluePrint/Core/Player/BP_PlayerAction.AimingEnemy` _playeractions))
  (bind _currentammo (`/Game/BluePrint/Core/Player/BP_PlayerAction.CurrentAmmo` _playeractions_4))
  (bind _combatdebugwidget (`/Game/BluePrint/Core/Combat/BP_CombatSystem.CombatDebugWidget` (`/Game/BluePrint/Core/Player/BP_PlayerAction.CombatSystem` _playeractions_3)))
  (`/Engine/EditorBlueprintResources/StandardMacros.IsValid` (`/Game/BluePrint/Core/Player/BP_PlayerAction.PlayerUnit` _playeractions)
    (:`Is Valid`
      (if (not (`/Game/BluePrint/Core/Player/BP_PlayerAction.IsReloadingWeaponAmmo` _playeractions_4))
        (`|ExecutionSequence`
          (:`then_0`
            (if (> _currentammo 0)
              (`/Engine/EditorBlueprintResources/StandardMacros.DecrementInt` _currentammo
                (:`  `
                  (`/Engine/EditorBlueprintResources/StandardMacros.IsValid` _combatdebugwidget
                    (:`Is Valid`
                      (`/Game/BluePrint/Core/Combat/DebugWidget/WBP_DebugCombatScreen.UpdateCurrentAmmo` _combatdebugwidget (`/Game/BluePrint/Core/Player/BP_PlayerAction.CurrentAmmo` _playeractions_3) (`/Game/BluePrint/Core/Player/BP_PlayerAction.MaxAmmo` _playeractions_3)))
                    (:`Is Not Valid`
                      _))
                  (if (<= (`/Game/BluePrint/Core/Player/BP_PlayerAction.CurrentAmmo` _playeractions_2) 0)
                    (set `/Game/BluePrint/Core/Player/BP_PlayerAction.CurrentAmmo` 0 _playeractions_2)
                    (`/Game/BluePrint/Core/Player/BP_PlayerAction.StartTimerToReloadWeaponAmmo` (`self.PlayerActions`)))))))
          (:`then_1`
            (`/Engine/EditorBlueprintResources/StandardMacros.IsValid` _aimingenemy
              (:`Is Valid`
                (`KismetSystemLibrary.PrintString` (`KismetStringLibrary.Concat_StrStr` "Aim Enemy" (`KismetSystemLibrary.GetDisplayName` _aimingenemy)) false true (struct :`R` 0.746026 :`B` 1.0 :`A` 1.0))
                (`/Game/BluePrint/Core/Character/BP_UnitMaster_Enemy.ModifierCurrentHp` _aimingenemy -2.0)))))))))

(fn `UserConstructionScript`
  (`parent.UserConstructionScript`))