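; Player action that builds or removes a tower on the selected terrain tiles and side tiles.
; When adding, it checks that the terrain is buildable, the tile suits the tower type, and coins cover the cost unless free building is enabled.
; It then removes any existing towers, spawns a BP_Tower and registers it with the CombatSystem, carrying over range rotation.
; Removal mode reuses the same removal step, which destroys the towers.
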(fn `ExecuteAction`
  (params (TerrainIndexAndSideTileIndex :type "Map of IntVector Structure to Integer"))
  (bind _playeractions (`self.PlayerActions`))
  (bind _playeractions_2 (`self.PlayerActions`))
  (bind _hoveredtower (`/Game/BluePrint/Core/Player/BP_PlayerAction.HoveredTower` _playeractions_2))
  (bind _combatsystem (`/Game/BluePrint/Core/Player/BP_PlayerAction.CombatSystem` (`self.PlayerActions`)))
  (if (`self.IsAddingTower`)
    ; Terrain Index 能不能建造
    (bind _keys (`BlueprintMapLibrary.Map_Keys` (`local.TerrainIndexAndSideTileIndex`)))
    (if (`/Game/BluePrint/Core/Terrain/BP_Terrain.IsTerrainIndexGroupAllTowerBuildable` (`/Game/BluePrint/Core/Player/BP_PlayerAction.Terrain` (`self.PlayerActions`)) _keys)
      ; Tile Side Index 符不符合该防御塔可建造的地砖类型
      (if (`/Game/BluePrint/Core/Combat/BP_CombatSystem.IsTowerBuildableOnTargetTileIndex` (`/Game/BluePrint/Core/Player/BP_PlayerAction.CombatSystem` (`self.PlayerActions`)) (`local.TerrainIndexAndSideTileIndex`) (`self.TowerType`))
        ; Comment
        (if (`/Game/BluePrint/Core/Combat/BP_CombatSystem.IsAbleToBuildingTowerWithoutCoins` _combatsystem)
          (`|ExecutionSequence` :!label _label
            (:`then_0`
              (bind _keys_2 (`BlueprintMapLibrary.Map_Keys` (`local.TerrainIndexAndSideTileIndex`) :!label _label_2))
              (for _array_element _keys_2
                (bind _values (`BlueprintMapLibrary.Map_Values` (`local.TerrainIndexAndSideTileIndex`)))
                (bind _value (`BlueprintMapLibrary.Map_Find` (`.TowerOnSideTile_28_CD3C8427467A2C9D9223D5932B9C9EDF` (break `/Game/BluePrint/Core/Terrain/Utilities/S_TileData` (`BlueprintMapLibrary.Map_Find` (`/Game/BluePrint/Core/Terrain/BP_Terrain.TerrainGridTiles` (`/Game/BluePrint/Core/Player/BP_PlayerAction.Terrain` (`self.PlayerActions`))) _array_element))) (`|GetArrayItem` _values)))
                (`/Engine/EditorBlueprintResources/StandardMacros.IsValid` _value
                  (:`Is Valid`
                    (if (`KismetSystemLibrary.IsValid` (`/Game/BluePrint/Core/Player/BP_PlayerAction.HoveredTower` (`self.PlayerActions`)))
                      (bind _output_get (set `/Game/BluePrint/Core/Player/BP_PlayerAction.Current_IsRotateRange` (`/Game/BluePrint/Core/Tower/BP_Tower.IsCurrentTowerRotate` _value) _playeractions))
                      (set `/Game/BluePrint/Core/Player/BP_PlayerAction.Record_IsRotateRange` _output_get _playeractions))
                    (`/Game/BluePrint/Core/Combat/BP_CombatSystem.RemoveTowerInCombat` (`/Game/BluePrint/Core/Player/BP_PlayerAction.CombatSystem` (`self.PlayerActions`)) _value true))
                  (:`Is Not Valid`
                    (`KismetSystemLibrary.PrintString` (`KismetStringLibrary.Concat_StrStr` "RemoveNotValidTower" (`KismetStringLibrary.Conv_IntVectorToString` _array_element)) true true (struct :`R` 1.0 :`B` 0.047016 :`A` 1.0) 5.0)))))
            (:`then_1`
              (bind _returnvalue (`|SpawnActorFromClass` "/Game/BluePrint/Core/Tower/BP_Tower.BP_Tower_C" (`KismetMathLibrary.MakeTransform` (0.0 0.0 0.0)) "Undefined" "MultiplyWithRoot" null (`self.TowerType`) (`/Game/BluePrint/Core/Terrain/BP_Terrain.TerrainGridSize` (`/Game/BluePrint/Core/Player/BP_PlayerAction.Terrain` (`self.PlayerActions`))) false null))
              (`/Game/BluePrint/Core/Combat/BP_CombatSystem.AddTowerInCombat` (`/Game/BluePrint/Core/Player/BP_PlayerAction.CombatSystem` _playeractions_2) _returnvalue (`local.TerrainIndexAndSideTileIndex`) (select `bool` (and (`KismetSystemLibrary.IsValid` _hoveredtower) (`/Game/BluePrint/Core/Player/BP_PlayerAction.IsNewHoveredTileIndexesComeFromTower` _playeractions_2)) :`false` (`/Game/BluePrint/Core/Player/BP_PlayerAction.Current_IsRotateRange` _playeractions_2) :`true` (`/Game/BluePrint/Core/Tower/BP_Tower.IsCurrentTowerRotate` _hoveredtower)))))
          (elif (>= (`.Coin_Current_28_0B062446407DD0E9A2F7E8A59BFCC10A` (break `/Game/BluePrint/Core/Combat/Utilities/S_CombatData` (`/Game/BluePrint/Core/Combat/BP_CombatSystem.CombatData` _combatsystem))) (`KismetMathLibrary.Abs_Int` (`.BuildCost_10_B13D469B4EDF07267921BD8B6F29D5D3` (break `/Game/BluePrint/Core/Tower/Utilities/S_TowerData_Stats_Numerical` (`.Stats_32_516A75554717573F9FE51BA7807FAD22` (break `/Game/BluePrint/Core/Tower/Utilities/S_DefenseTowerData` (`/Game/BluePrint/Core/Tower/Utilities/BFL_Towers.GetDefaultTowerDataBaseOnTowerType` (`self.TowerType`))))))))
            (goto _label)))))
    (else
      (goto _label_2))))

(fn `UserConstructionScript`
  (`parent.UserConstructionScript`))