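; Player action that upgrades the tower on the hovered terrain tile by one level.
; ExecuteAction loops the passed terrain indices, looks up each tower using the first side-tile value, and checks the combat system's upgrade permission.
; Level cap and cost come from default data for the tower type, not the tower instance.
; A DoOnce gates the upgrade, which requires and applies the coin cost unless free upgrades are enabled.
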(fn `ExecuteAction`
  (params (TerrainIndexAndSideTileIndex :type "Map of IntVector Structure to Integer"))
  (locals (CurrentTowerType :type "/Game/BluePrint/Core/Tower/Utilities/Enum_TowerType Enum" :default "NewEnumerator8"))
  (bind _terrainindexandsidetileindex (`local.TerrainIndexAndSideTileIndex`))
  (bind _combatsystem (`/Game/BluePrint/Core/Player/BP_PlayerAction.CombatSystem` (`self.PlayerActions`)))
  (bind ((`CurrentLevel_11_40A8CAEF4711C73A6E7C9E967904F26E` _currentlevel) (`Level_UpgradeCost_50_6733FF4D4A45895C688BF5BD8A42B08B` _level_upgradecost)) (break `/Game/BluePrint/Core/Tower/Utilities/S_TowerData_Stats_Numerical` (`.Stats_32_516A75554717573F9FE51BA7807FAD22` (break `/Game/BluePrint/Core/Tower/Utilities/S_DefenseTowerData` (`/Game/BluePrint/Core/Tower/Utilities/BFL_Towers.GetDefaultTowerDataBaseOnTowerType` (`local.CurrentTowerType`))))))
  (bind ((`MaxLevel_12_3C3A3FCC4DAA468E51D6F1BC1FD8198C` _maxlevel) (`CurrentLevel_11_40A8CAEF4711C73A6E7C9E967904F26E` _currentlevel_2) (`Level_UpgradeCost_50_6733FF4D4A45895C688BF5BD8A42B08B` _level_upgradecost_2)) (break `/Game/BluePrint/Core/Tower/Utilities/S_TowerData_Stats_Numerical` (`.Stats_32_516A75554717573F9FE51BA7807FAD22` (break `/Game/BluePrint/Core/Tower/Utilities/S_DefenseTowerData` (`/Game/BluePrint/Core/Tower/Utilities/BFL_Towers.GetDefaultTowerDataBaseOnTowerType` (`local.CurrentTowerType`))))))
  (if (> (`BlueprintMapLibrary.Map_Length` _terrainindexandsidetileindex) 0)
    (bind _keys (`BlueprintMapLibrary.Map_Keys` _terrainindexandsidetileindex))
    (for _array_element _keys
      (bind _values (`BlueprintMapLibrary.Map_Values` (`local.TerrainIndexAndSideTileIndex`)))
      (bind _value (`BlueprintMapLibrary.Map_Find` (`.TowerOnSideTile_28_CD3C8427467A2C9D9223D5932B9C9EDF` (break `/Game/BluePrint/Core/Terrain/Utilities/S_TileData` (`BlueprintMapLibrary.Map_Find` (`/Game/BluePrint/Core/Terrain/BP_Terrain.TerrainGridTiles` (`/Game/BluePrint/Core/Player/BP_PlayerAction.Terrain` (`self.PlayerActions`))) _array_element))) (`|GetArrayItem` _values)))
      (`/Engine/EditorBlueprintResources/StandardMacros.IsValid` _value
        (:`Is Valid`
          (if (`/Game/BluePrint/Core/Combat/BP_CombatSystem.IsAbleToUseTowerUpgradeInCurrentCombat` _combatsystem)
            (set `local.CurrentTowerType` (`/Game/BluePrint/Core/Tower/BP_Tower.TowerType` _value))
            (if (< _currentlevel_2 _maxlevel)
              (if (`/Game/BluePrint/Core/Combat/BP_CombatSystem.IsAbleToUpgradeTowerWithoutCoins` _combatsystem)
                (`/Engine/EditorBlueprintResources/StandardMacros.DoOnce` false :!label _label
                  (:`Completed`
                    (`/Game/BluePrint/Core/Tower/BP_Tower.ModifyTowerLevel` _value 1)
                    (if (not (`/Game/BluePrint/Core/Combat/BP_CombatSystem.IsAbleToUpgradeTowerWithoutCoins` (`/Game/BluePrint/Core/Player/BP_PlayerAction.CombatSystem` (`self.PlayerActions`))))
                      (`/Game/BluePrint/Core/Combat/BP_CombatSystem.ModifierCurrentCoin` (`/Game/BluePrint/Core/Player/BP_PlayerAction.CombatSystem` (`self.PlayerActions`)) (`BlueprintMapLibrary.Map_Find` _level_upgradecost _currentlevel)))))
                (elif (>= (`.CurrentCoins_10_47BDAEEA40A59310FA33559BD206058D` (break `/Game/BluePrint/Core/Combat/Utilities/S_Combat_Stats` (`.Stats_31_07E6A28149CDD8515CE29D8AE1A93512` (break `/Game/BluePrint/Core/Combat/Utilities/S_CombatData` (`/Game/BluePrint/Core/Combat/BP_CombatSystem.CombatData` (`/Game/BluePrint/Core/Player/BP_PlayerAction.CombatSystem` (`self.PlayerActions`))))))) (`KismetMathLibrary.Abs_Int` (`BlueprintMapLibrary.Map_Find` _level_upgradecost_2 _currentlevel_2)))
                  (goto _label))))))))))

(fn `UserConstructionScript`
  (`parent.UserConstructionScript`))