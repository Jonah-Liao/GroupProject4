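; Player action child Blueprint for selecting a terrain tile, currently left unwired so it changes nothing.
; ExecuteAction takes a terrain-index to side-index map and compares its first key with the stored selected tile, but neither branch continues.
; Disconnected nodes hold the intended logic: remove a state from the previous tile, store the new indices on PlayerActions, and add a state to the new tile.
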(fn `ExecuteAction`
  (params (TerrainIndexAndSideTileIndex :type "Map of IntVector Structure to Integer"))
  (bind _keys (`BlueprintMapLibrary.Map_Keys` (`local.TerrainIndexAndSideTileIndex`)))
  (if (not (`KismetMathLibrary.EqualExactly_VectorVector` (`KismetMathLibrary.Conv_IntVectorToVector` (`|GetArrayItem` _keys)) (`KismetMathLibrary.Conv_IntVectorToVector` (`/Game/BluePrint/Core/Player/BP_PlayerAction.SelectedTileIndex` (`self.PlayerActions`)))))
    _))

(fn `UserConstructionScript`
  (`parent.UserConstructionScript`))