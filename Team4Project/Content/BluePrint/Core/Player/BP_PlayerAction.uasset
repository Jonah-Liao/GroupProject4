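; Player controller-side tile interaction hub that hovers terrain tiles, runs click actions and can hand possession to the player unit.
; Each tick it asks BP_Terrain for the tile group and side under the cursor and moves the hover state to it.
; Left and right clicks execute swappable action actors, spawned by SetSelectedActions, on the hovered group.
; An input switches possession to BP_UnitMaster_Player, with delayed flags limiting switches both ways.
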(event `self.ReceiveBeginPlay`
  (bind _returnvalue (`GameplayStatics.GetPlayerController` 0))
  (bind _returnvalue_2 (pcsubsystem `EnhancedInputLocalPlayerSubsystem` _returnvalue))
  (`|ExecutionSequence`
    (:`then_0`
      (bind _returnvalue_3 (`GameplayStatics.GetActorOfClass` "/Game/BluePrint/Core/Terrain/BP_Terrain.BP_Terrain_C"))
      (set `self.Terrain` _returnvalue_3)
      (bind _returnvalue_4 (`GameplayStatics.GetActorOfClass` "/Game/BluePrint/Core/Character/BP_UnitMaster_Player.BP_UnitMaster_Player_C"))
      (bind _output_get (set `self.PlayerUnit` _returnvalue_4))
      (set `/Game/BluePrint/Core/Character/BP_UnitMaster_Player.PlayerAction` self _output_get)
      (add `/Game/BluePrint/Core/Character/BP_UnitMaster_Player.OnControllerSwitchToPawn` _output_get (`|CreateDelegate` :!event `OnControllerSwitchToPawn`))
      (bind _returnvalue_5 (`GameplayStatics.GetActorOfClass` "/Game/BluePrint/Core/Debug/BP_DebugMenu.BP_DebugMenu_C"))
      (set `self.DebugMenu` _returnvalue_5)
      (`/Engine/EditorBlueprintResources/StandardMacros.IsValid` _returnvalue_2
        (:`Is Valid`
          (`EnhancedInputSubsystemInterface.AddMappingContext` _returnvalue_2 "/Game/BluePrint/Core/Player/Input/IMC_PlayerAction.IMC_PlayerAction" 0 (struct))
          (`self.EnableInput` _returnvalue))))
    (:`then_1`
      (`self.ResetPlayerControllerState`))))

(event `self.ReceiveTick`
  (params (DeltaSeconds :type "Float (single-precision)"))
  (`self.UpdateTileStateUnderCursor` (`self.TileRange`)))

(event `EnhancedInput|/Game/BluePrint/Core/Player/Input/IA_MouseLeftClick`
  (params (ActionValue :type Boolean) (ElapsedSeconds :type "Float (double-precision)") (TriggeredSeconds :type "Float (double-precision)") (InputAction :type "InputAction Object Reference" :default "/Game/BluePrint/Core/Player/Input/IA_MouseLeftClick.IA_MouseLeftClick"))
  (:`Triggered`
    (if ActionValue
      (`/Engine/EditorBlueprintResources/StandardMacros.DoOnce` false :!label _label
        (:`Completed`
          (`self.UpdateTileStateUnderCursor` (`self.TileRange`))
          (`/Engine/EditorBlueprintResources/StandardMacros.IsValid` (`self.SelectAction_LeftClick`)
            (:`Is Valid`
              (`/Game/BluePrint/Core/Player/Actions/BP_Action.ExecuteAction` (`self.SelectAction_LeftClick`) (`self.HoveredTileIndexAndTileSideIndex`))))))))
  (:`Completed`
    (goto _label :!via `Reset`)))

(event `EnhancedInput|/Game/BluePrint/Core/Player/Input/IA_MouseRightClick`
  (params (ActionValue :type Boolean) (ElapsedSeconds :type "Float (double-precision)") (TriggeredSeconds :type "Float (double-precision)") (InputAction :type "InputAction Object Reference" :default "/Game/BluePrint/Core/Player/Input/IA_MouseRightClick.IA_MouseRightClick"))
  (:`Triggered`
    (if ActionValue
      (`/Engine/EditorBlueprintResources/StandardMacros.DoOnce` false :!label _label_2
        (:`Completed`
          (`self.UpdateTileStateUnderCursor` (`self.TileRange`))
          (`/Engine/EditorBlueprintResources/StandardMacros.IsValid` (`self.SelectAction_RightClick`)
            (:`Is Valid`
              (`/Game/BluePrint/Core/Player/Actions/BP_Action.ExecuteAction` (`self.SelectAction_RightClick`) (`self.HoveredTileIndexAndTileSideIndex`))))))))
  (:`Completed`
    (goto _label_2 :!via `Reset`)))

(event `EnhancedInput|/Game/BluePrint/Core/Player/Input/IA_ControllerPossessSwitch`
  (params (ActionValue :type Boolean) (ElapsedSeconds :type "Float (double-precision)") (TriggeredSeconds :type "Float (double-precision)") (InputAction :type "InputAction Object Reference" :default "/Game/BluePrint/Core/Player/Input/IA_ControllerPossessSwitch.IA_ControllerPossessSwitch"))
  (bind _playerunit (`self.PlayerUnit`))
  (bind _controllercurrentstate (`self.ControllerCurrentState`))
  (:`Triggered`
    (if ActionValue
      (if (and (`|EnumInequality` _controllercurrentstate "NewEnumerator1") (`|EnumInequality` _controllercurrentstate "NewEnumerator2") (`self.IsPlayerActionAbleToSwitchPossess`))
        (`/Engine/EditorBlueprintResources/StandardMacros.IsValid` _playerunit
          (:`Is Valid`
            (`Controller.Possess` (`GameplayStatics.GetPlayerController` 0) _playerunit)
            (`self.SetPlayerControllerState` "NewEnumerator1")
            (`KismetSystemLibrary.Delay` 3.0)
            (set `/Game/BluePrint/Core/Character/BP_UnitMaster_Player.IsAbleToSwitchPossess` true (`self.PlayerUnit`))
            (set `self.IsPlayerActionAbleToSwitchPossess` false)))))))

(event `OnControllerSwitchToPawn`
  (`self.SetPlayerControllerState` "NewEnumerator0")
  (`KismetSystemLibrary.Delay` 3.0)
  (set `self.IsPlayerActionAbleToSwitchPossess` true))

(fn `ResetPlayerControllerState`
  (`/Engine/EditorBlueprintResources/StandardMacros.IsValid` (`self.DebugMenu`)
    (:`Is Valid`
      (set `self.ControllerCurrentState` "NewEnumerator0")
      (set `self.IsPlayerActionAbleToSwitchPossess` true))
    (:`Is Not Valid`
      (`/Engine/EditorBlueprintResources/StandardMacros.IsValid` (`self.PlayerUnit`)
        (:`Is Valid`
          (set `self.ControllerCurrentState` "NewEnumerator1"))
        (:`Is Not Valid`
          (set `self.ControllerCurrentState` "NewEnumerator0"))))))

(fn `SetPlayerControllerState`
  (params (ControllerCurrentState :type "/Game/BluePrint/Core/Player/Utilities/Enum_ControllerState Enum" :default "NewEnumerator0"))
  (set `self.ControllerCurrentState` ControllerCurrentState))

(fn `SetSelectedActions`
  (params (LeftAction :type "/Game/BluePrint/Core/Player/Actions/BP_Action Class Reference") (RightAction :type "/Game/BluePrint/Core/Player/Actions/BP_Action Class Reference"))
  (bind _selectaction_leftclick (`self.SelectAction_LeftClick`))
  (bind _selectaction_rightclick (`self.SelectAction_RightClick`))
  (`|ExecutionSequence`
    (:`then_0`
      (`/Engine/EditorBlueprintResources/StandardMacros.IsValid` _selectaction_leftclick
        (:`Is Valid`
          (`self.K2_DestroyActor` _selectaction_leftclick)
          (set `self.SelectAction_LeftClick` null))
        (:`Is Not Valid`
          _))
      (if (`KismetSystemLibrary.IsValidClass` (`local.LeftAction`))
        (bind _returnvalue (`|SpawnActorFromClass` (`local.LeftAction`) (`KismetMathLibrary.MakeTransform` (0.0 0.0 0.0)) "AlwaysSpawn" "MultiplyWithRoot" null self null))
        (set `self.SelectAction_LeftClick` _returnvalue)))
    (:`then_1`
      (`/Engine/EditorBlueprintResources/StandardMacros.IsValid` _selectaction_rightclick
        (:`Is Valid`
          (`self.K2_DestroyActor` _selectaction_rightclick)
          (set `self.SelectAction_RightClick` null))
        (:`Is Not Valid`
          _))
      (if (`KismetSystemLibrary.IsValidClass` (`local.RightAction`))
        (bind _returnvalue_2 (`|SpawnActorFromClass` (`local.RightAction`) (`KismetMathLibrary.MakeTransform` (0.0 0.0 0.0)) "AlwaysSpawn" "MultiplyWithRoot" null self null))
        (set `self.SelectAction_RightClick` _returnvalue_2)))
    (:`then_2`
      (`self.OnSelectedActionsChanged` (`self.SelectAction_LeftClick`) (`self.SelectAction_RightClick`)))))

(fn `UpdateTileStateUnderCursor`
  (params (TileCount :type "IntPoint Structure"))
  (locals (NewHoveredTileIndex :type "IntVector Structure") (NewSideIndex :type Integer :default 0))
  (bind _hoveredtileindexandtilesideindex (`self.HoveredTileIndexAndTileSideIndex`))
  (bind (_tileindex _sideindex) (`/Game/BluePrint/Core/Terrain/BP_Terrain.GetTileIndexAndSideIndexUnderCursor` (`self.Terrain`) 0 false (`self.PlayerUnit`)))
  (set `local.NewHoveredTileIndex` _tileindex)
  (set `local.NewSideIndex` _sideindex)
  (if (> (`BlueprintMapLibrary.Map_Length` (`self.HoveredTileIndexAndTileSideIndex`)) 0)
    (bind _values (`BlueprintMapLibrary.Map_Values` _hoveredtileindexandtilesideindex))
    (bind _keys (`BlueprintMapLibrary.Map_Keys` _hoveredtileindexandtilesideindex))
    (if (and (or (`KismetMathLibrary.NotEqualExactly_VectorVector` (`KismetMathLibrary.Conv_IntVectorToVector` (`local.NewHoveredTileIndex`)) (`KismetMathLibrary.Conv_IntVectorToVector` (`|GetArrayItem` _keys))) (!= (`local.NewSideIndex`) (`|GetArrayItem` _values))) (`.ReturnValue` (`BlueprintMapLibrary.Map_Find` (`/Game/BluePrint/Core/Terrain/BP_Terrain.TerrainGridTiles` (`self.Terrain`)) (`local.NewHoveredTileIndex`))))
      (bind (_targettilesgroup _isfindtilessuccessfully) (`/Game/BluePrint/Core/Terrain/BP_Terrain.GetPossibleTilesGroupBaseOnSingleTile` (`self.Terrain`) (`local.NewHoveredTileIndex`) (`local.NewSideIndex`) (`local.TileCount`) true :!label _label))
      (if (> (`BlueprintMapLibrary.Map_Length` (`self.HoveredTileIndexAndTileSideIndex`)) 0)
        (`/Game/BluePrint/Core/Terrain/BP_Terrain.RemoveStateFromTilesGroup` (`self.Terrain`) (`self.HoveredTileIndexAndTileSideIndex`) "NewEnumerator1"))
      (if _isfindtilessuccessfully
        (set `self.HoveredTileIndexAndTileSideIndex` _targettilesgroup)
        (`/Game/BluePrint/Core/Terrain/BP_Terrain.AddStateToTilesGroup` (`self.Terrain`) (`self.HoveredTileIndexAndTileSideIndex`) "NewEnumerator1")))
    (elif (`.ReturnValue` (`BlueprintMapLibrary.Map_Find` (`/Game/BluePrint/Core/Terrain/BP_Terrain.TerrainGridTiles` (`self.Terrain`)) (`local.NewHoveredTileIndex`)))
      (goto _label))))

(fn `UserConstructionScript`)